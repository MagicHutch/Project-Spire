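; BP_TestIntersectionBreakableObject is a test actor that breaks when struck hard enough by a BP_TestIntersectionObject.
; Its Cube's hit event casts the other actor to that class and compares the length of the normal impulse to a hardcoded threshold.
; Impacts above the threshold destroy the actor outright, with no fracture or effects, and debug strings print each outcome.
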(event `self.Cube.OnComponentHit`
  (params (HitComponent :type "PrimitiveComponent Object Reference") (OtherActor :type "Actor Object Reference") (OtherComp :type "PrimitiveComponent Object Reference") (NormalImpulse :type "Vector Structure") (Hit :type "HitResult Structure (by ref)"))
  (`KismetSystemLibrary.PrintString` "break")
  (cast `/Game/Blueprints/IntersectionObjects/BP_TestIntersectionObject` OtherActor
    (:`then`
      (`KismetSystemLibrary.PrintString` (`KismetStringLibrary.Conv_VectorToString` NormalImpulse))
      (if (> (`KismetMathLibrary.VSize` NormalImpulse) 150000.0)
        (`KismetSystemLibrary.PrintString` "objectBroken")
        (`self.K2_DestroyActor`)
        (else
          (`KismetSystemLibrary.PrintString` "objectNotBroken"))))
    (:`CastFailed`
      (`KismetSystemLibrary.PrintString` "not an intersection object"))))

(fn `UserConstructionScript`)