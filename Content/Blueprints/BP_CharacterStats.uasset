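; BP_CharacterStats is a Blueprint that tracks a character's health and stamina.
; On BeginPlay it fills both current values to their maximums.
; Each Tick it regenerates stamina at a per-second rate scaled by frame time and clamped to the maximum, while health has no regeneration.
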(event `self.ReceiveBeginPlay`
  (set `self.CurrentHealth` (`self.MaxHealth`))
  (set `self.CurrentStamina` (`self.MaxStamina`)))

(event `self.ReceiveTick`
  (params (DeltaSeconds :type "Float (single-precision)"))
  (if (< (`self.CurrentStamina`) (`self.MaxStamina`))
    (set `self.CurrentStamina` (`KismetMathLibrary.FClamp` (+ (`self.CurrentStamina`) (* (`self.StaminaPerSecond`) DeltaSeconds)) 0.0 (`self.MaxStamina`)))))