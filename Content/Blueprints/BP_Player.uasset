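; Player character with Enhanced Input movement, roll dodge, enemy lock-on and stamina-gated weapon attacks.
; BeginPlay collects the level's weapons into Inventory and equips a random one to a hand bone key, which Tick follows by repositioning the actor.
; Lock-on snapshots the transform of the on-screen "Enemy" actor nearest screen centre, and Tick turns control rotation toward it.
; Attack montage notifies toggle the weapon's attack window.
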(event `self.ReceiveBeginPlay`
  ;[1 1 1] Begin
  (`EnhancedInputSubsystemInterface.AddMappingContext` (pcsubsystem `EnhancedInputLocalPlayerSubsystem` (`GameplayStatics.GetPlayerController` 0)) "/Game/ThirdPerson/Input/IMC_Default.IMC_Default" 0 (struct))
  (bind _outactors (`GameplayStatics.GetAllActorsOfClass` "/Game/Blueprints/Weapons/BP_WeaponClass.BP_WeaponClass_C"))
  (for _array_element _outactors
    (`KismetArrayLibrary.Array_Add` (`self.Inventory`) _array_element)
    (`BlueprintMapLibrary.Map_Add` (`self.Equipment`) "Bone_008" (`KismetArrayLibrary.Array_Random` (`self.Inventory`)))
    (for _array_element_2 (`self.Inventory`)
      (bind _values (`BlueprintMapLibrary.Map_Values` (`self.Equipment`)))
      (if (not true)
        (`self.SetActorHiddenInGame` _array_element_2 true)))))

(event `EnhancedInput|/Game/ThirdPerson/Input/Actions/IA_Move`
  (params (ActionValue :type "Vector2D Structure") (ElapsedSeconds :type "Float (double-precision)") (TriggeredSeconds :type "Float (double-precision)") (InputAction :type "InputAction Object Reference" :default "/Game/ThirdPerson/Input/Actions/IA_Move.IA_Move"))
  (bind (_returnvalue_roll _returnvalue_pitch _returnvalue_yaw) (`KismetMathLibrary.BreakRotator` (`self.GetControlRotation`)))
  (bind (_returnvalue_roll_2 _returnvalue_pitch_2 _returnvalue_yaw_2) (`KismetMathLibrary.BreakRotator` (`self.GetControlRotation`)))
  ;[1 1 1] Move Logic
  (:`Triggered`
    (`self.AddMovementInput` (`KismetMathLibrary.GetRightVector` (`KismetMathLibrary.MakeRotator` _returnvalue_roll_2 0.0 _returnvalue_yaw_2)) ActionValue_X)
    (`self.AddMovementInput` (`KismetMathLibrary.GetForwardVector` (`KismetMathLibrary.MakeRotator` _returnvalue_roll 0.0 _returnvalue_yaw)) ActionValue_Y)))

(event `self.ReceiveTick`
  (params (DeltaSeconds :type "Float (single-precision)"))
  ;[1 1 1] Tick
  (`self.LockOn Logic`)
  (`self.Update Equipment`))

(event `EnhancedInput|/Game/ThirdPerson/Input/Actions/IA_Look`
  (params (ActionValue :type "Vector2D Structure") (ElapsedSeconds :type "Float (double-precision)") (TriggeredSeconds :type "Float (double-precision)") (InputAction :type "InputAction Object Reference" :default "/Game/ThirdPerson/Input/Actions/IA_Look.IA_Look"))
  ;[1 1 1] Look Logic
  (:`Triggered`
    (`self.AddControllerYawInput` ActionValue_X)
    (`self.AddControllerPitchInput` ActionValue_Y)))

(event `EnhancedInput|/Game/ThirdPerson/Input/Actions/IA_LockOn`
  (params (ActionValue :type Boolean) (ElapsedSeconds :type "Float (double-precision)") (TriggeredSeconds :type "Float (double-precision)") (InputAction :type "InputAction Object Reference" :default "/Game/ThirdPerson/Input/Actions/IA_LockOn.IA_LockOn"))
  ;[1 1 1] LockOn Init
  (:`Triggered`
    (`self.Init LockOn`)))

(event `LockOn Logic`
  (bind _returnvalue_location (`KismetMathLibrary.BreakTransform` (`self.GetTransform`)))
  (bind _lockon_transform_location (`KismetMathLibrary.BreakTransform` (`self.LockOn Transform`)))
  (bind (_yaw _pitch) (`KismetMathLibrary.GetYawPitchFromVector` (`KismetMathLibrary.Normal` (- _lockon_transform_location _returnvalue_location))))
  ;[1 1 1] LockOn Logic
  (if (`self.Is LockOn`)
    (`Controller.SetControlRotation` (`GameplayStatics.GetPlayerController` 0) (`KismetMathLibrary.MakeRotator` 0.0 _pitch _yaw))))

(event `Init LockOn`
  (bind _returnvalue (`WidgetLayoutLibrary.GetViewportSize`))
  (bind _lockon_options (`self.LockOn Options`))
  ;[1 1 1] LockOn Init
  (if (`self.Is LockOn`)
    (set `self.Is LockOn` false)
    (else
      ;;[1 1 1] Is there an enemy list to check
      (bind _outactors (`GameplayStatics.GetAllActorsWithTag` "Enemy"))
      (if (> (`KismetArrayLibrary.Array_Length` _outactors) 0)
        (`BlueprintMapLibrary.Map_Clear` (`self.LockOn Options`))
        (for _array_element _outactors
          (bind _returnvalue_location (`KismetMathLibrary.BreakTransform` (`self.GetTransform` _array_element)))
          (bind _screenposition (`GameplayStatics.ProjectWorldToScreen` (`GameplayStatics.GetPlayerController` 0) _returnvalue_location))
          (bind _returnvalue_2 (`self.IsOnScreen` _returnvalue _screenposition))
          (if _returnvalue_2
            (`BlueprintMapLibrary.Map_Add` (`self.LockOn Options`) (`self.GetTransform` _array_element) (`KismetMathLibrary.Distance2D` (/ _returnvalue 2.0) _screenposition))))
        (bind _keys (`BlueprintMapLibrary.Map_Keys` (`self.LockOn Options`)))
        (set `self.LockOn Transform` (`|GetArrayItem` _keys))
        (for _array_element_2 _keys
          (if (< (`BlueprintMapLibrary.Map_Find` _lockon_options _array_element_2) (`BlueprintMapLibrary.Map_Find` _lockon_options (`self.LockOn Transform`)))
            (set `self.LockOn Transform` _array_element_2)))
        (set `self.Is LockOn` true)))))

(event `Update Equipment`
  (bind _equipment (`self.Equipment`))
  ;[1 1 1] Update Equipment
  (bind _keys (`BlueprintMapLibrary.Map_Keys` _equipment))
  (for _array_element _keys
    (bind _value (`BlueprintMapLibrary.Map_Find` _equipment _array_element))
    (if (!= _value null)
      (bind (_returnvalue_location _returnvalue_rotation) (`KismetMathLibrary.BreakTransform` (`SkinnedMeshComponent.GetBoneTransform` (`self.Mesh`) _array_element "RTS_World")))
      (`self.K2_SetActorLocationAndRotation` _value (+ _returnvalue_location (* (`KismetMathLibrary.GetRightVector` _returnvalue_rotation) -10.0)) _returnvalue_rotation false false))))

(event `EnhancedInput|/Game/ThirdPerson/Input/Actions/IA_Dodge`
  (params (ActionValue :type Boolean) (ElapsedSeconds :type "Float (double-precision)") (TriggeredSeconds :type "Float (double-precision)") (InputAction :type "InputAction Object Reference" :default "/Game/ThirdPerson/Input/Actions/IA_Dodge.IA_Dodge"))
  ;[1 1 1] Dodge
  (:`Completed`
    (`|PlayMontage` (`self.Mesh`) "/Game/Characters/PlayerV2/Animations/MediumRoll.MediumRoll")))

(event `EnhancedInput|/Game/ThirdPerson/Input/Actions/IA_RightAttack`
  (params (ActionValue :type Boolean) (ElapsedSeconds :type "Float (double-precision)") (TriggeredSeconds :type "Float (double-precision)") (InputAction :type "InputAction Object Reference" :default "/Game/ThirdPerson/Input/Actions/IA_RightAttack.IA_RightAttack"))
  (bind _bp_characterstats (`self.BP_CharacterStats`))
  (bind _value (`BlueprintMapLibrary.Map_Find` (`self.Equipment`) "Bone_008"))
  (bind _staminacost (`/Game/Blueprints/Weapons/BP_WeaponClass.StaminaCost` _value))
  ;[1 1 1] Attack Logic
  (:`Started`
    (if (>= (`/Game/Blueprints/BP_CharacterStats.CurrentStamina` (`self.BP_CharacterStats`)) _staminacost)
      (if (`self.CanAttack`)
        (set `/Game/Blueprints/BP_CharacterStats.CurrentStamina` (- (`/Game/Blueprints/BP_CharacterStats.CurrentStamina` _bp_characterstats) _staminacost) _bp_characterstats)
        (`|PlayMontage` (`self.Mesh`) (`|GetArrayItem` (`/Game/Blueprints/Weapons/BP_WeaponClass.AnimationMontage` _value))
          (:`then`
            (set `self.CanAttack` false))
          (:`OnCompleted`
            (set `self.CanAttack` true))
          (:`OnNotifyBegin`
            (`/Game/Blueprints/Weapons/BP_WeaponClass.Activate Attack` _value))
          (:`OnNotifyEnd`
            (`/Game/Blueprints/Weapons/BP_WeaponClass.Deactivate Attack` _value)
            (`self.StopAnimMontage` null)
            (set `self.CanAttack` true)))))))

(fn `UserConstructionScript`)