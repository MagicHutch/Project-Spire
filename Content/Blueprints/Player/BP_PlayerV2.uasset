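; Player character Blueprint for an action game with stamina-gated actions, lock-on targeting, item pickups and an inventory menu.
; Dodge, attack and damage reactions are action objects run through NextState, which spends stamina and sets the current state.
; Tick regenerates stamina, allows input only in the base state with the menu closed, and turns the controller toward the lock target.
; Lock-on picks the on-screen Enemy-tagged actor nearest screen centre.
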(event `self.ReceiveBeginPlay`
  (bind _returnvalue (`GameplayStatics.GetPlayerController` 0))
  (bind _bp_playerinventory (`self.BP_PlayerInventory`))
  ;[1 1 1] Begin
  ;;[1 1 1] Configure Input
  (`EnhancedInputSubsystemInterface.AddMappingContext` (pcsubsystem `EnhancedInputLocalPlayerSubsystem` _returnvalue) "/Game/ThirdPerson/Input/IMC_Default.IMC_Default" 0 (struct))
  (`WidgetBlueprintLibrary.SetInputMode_GameOnly` _returnvalue)
  ;;[1 1 1] Create UI
  (bind _returnvalue_2 (`|CreateWidget` "/Game/UI/WB_PlayerStats.WB_PlayerStats_C"))
  (bind _output_get (set `self.UI` _returnvalue_2))
  (`UserWidget.AddToViewport` _output_get 0)
  (`/Game/UI/WB_PlayerStats.Fill Inventory` _output_get (`/Game/Blueprints/Player/BP_PlayerInventory.WeaponList` _bp_playerinventory) (`/Game/Blueprints/Player/BP_PlayerInventory.ConsumableList` _bp_playerinventory))
  ;;[1 1 1] Action Logic
  (`self.InitializeActionList`)
  (bind _output_get_2 (set `self.CurrentState` (`BlueprintMapLibrary.Map_Find` (`self.StateList`) "NewEnumerator0")))
  (`self.NextState` _output_get_2))

(event `self.ReceiveTick`
  (params (DeltaSeconds :type "Float (single-precision)"))
  (`self.UpdateStamina` DeltaSeconds)
  (`self.UpdateCanAct`)
  (`self.LockOn Logic`))

(event `EnhancedInput|/Game/ThirdPerson/Input/Actions/IA_Look`
  (params (ActionValue :type "Vector2D Structure") (ElapsedSeconds :type "Float (double-precision)") (TriggeredSeconds :type "Float (double-precision)") (InputAction :type "InputAction Object Reference" :default "/Game/ThirdPerson/Input/Actions/IA_Look.IA_Look"))
  ;[1 1 1] Look Logic
  (:`Triggered`
    (if (`self.CanAct`)
      (`self.AddControllerYawInput` ActionValue_X)
      (`self.AddControllerPitchInput` ActionValue_Y))))

(event `LockOn Logic`
  (bind _returnvalue_location (`KismetMathLibrary.BreakTransform` (`self.GetTransform`)))
  (bind _lockontarget (`self.LockOnTarget`))
  (bind (_yaw _pitch) (`KismetMathLibrary.GetYawPitchFromVector` (`KismetMathLibrary.Normal` (- (+ (`self.K2_GetActorLocation` _lockontarget) (`EnemyCharacter.lockOnOffset` _lockontarget)) _returnvalue_location))))
  ;[1 1 1] LockOn Logic
  (if (`KismetSystemLibrary.IsValid` (`self.LockOnTarget`))
    (`Controller.SetControlRotation` (`GameplayStatics.GetPlayerController` 0) (`KismetMathLibrary.MakeRotator` 0.0 _pitch _yaw))))

(event `EnhancedInput|/Game/ThirdPerson/Input/Actions/IA_Dodge`
  (params (ActionValue :type Boolean) (ElapsedSeconds :type "Float (double-precision)") (TriggeredSeconds :type "Float (double-precision)") (InputAction :type "InputAction Object Reference" :default "/Game/ThirdPerson/Input/Actions/IA_Dodge.IA_Dodge"))
  ;[1 1 1] Dodge Logic
  (:`Triggered`
    (if (`self.CanAct`)
      (`self.NextState` (`self.PA_Dodge`)))))

(event `EnhancedInput|/Game/ThirdPerson/Input/Actions/IA_RightAttack`
  (params (ActionValue :type Boolean) (ElapsedSeconds :type "Float (double-precision)") (TriggeredSeconds :type "Float (double-precision)") (InputAction :type "InputAction Object Reference" :default "/Game/ThirdPerson/Input/Actions/IA_RightAttack.IA_RightAttack"))
  ;[1 1 1] RightAttack Logic
  (:`Triggered`
    (if (`self.CanAct`)
      (`self.NextState` (`self.PA_RightAttack`)))))

(event `EnhancedInput|/Game/ThirdPerson/Input/Actions/IA_LockOn`
  (params (ActionValue :type Boolean) (ElapsedSeconds :type "Float (double-precision)") (TriggeredSeconds :type "Float (double-precision)") (InputAction :type "InputAction Object Reference" :default "/Game/ThirdPerson/Input/Actions/IA_LockOn.IA_LockOn"))
  ;[1 1 1] LockOn Init Logic
  (:`Triggered`
    (if (`self.CanAct`)
      (if (`KismetSystemLibrary.IsValid` (`self.LockOnTarget`))
        (set `self.LockOnTarget` null)
        (set `self.bUseControllerRotationYaw` false)
        (else
          (`self.FindLockOnTarget`)
          (set `self.bUseControllerRotationYaw` true))))))

(event `EnhancedInput|/Game/ThirdPerson/Input/Actions/IA_Interact`
  (params (ActionValue :type Boolean) (ElapsedSeconds :type "Float (double-precision)") (TriggeredSeconds :type "Float (double-precision)") (InputAction :type "InputAction Object Reference" :default "/Game/ThirdPerson/Input/Actions/IA_Interact.IA_Interact"))
  (bind _bp_playerinventory (`self.BP_PlayerInventory`))
  (bind _bp_playerinventory_2 (`self.BP_PlayerInventory`))
  (bind _interactobject (`self.InteractObject`))
  (bind _weaponlist (`/Game/Blueprints/Player/BP_PlayerInventory.WeaponList` _bp_playerinventory))
  (bind _itemtogive (`/Game/Blueprints/Items/BP_ItemPickup.ItemToGive` _interactobject))
  (bind _consumablelist (`/Game/Blueprints/Player/BP_PlayerInventory.ConsumableList` _bp_playerinventory))
  ;[1 1 1] Interact Logic
  (:`Triggered`
    (if (`self.CanAct`)
      (if (!= _interactobject null)
        (bind _asusable_weapon (castclass `UsableWeapon` _itemtogive)
          (:`then`
            (if (`BlueprintMapLibrary.Map_Contains` _weaponlist _asusable_weapon)
              (`BlueprintMapLibrary.Map_Add` _weaponlist _asusable_weapon (+ (`BlueprintMapLibrary.Map_Find` _weaponlist _asusable_weapon) 1))
              (else
                (`BlueprintMapLibrary.Map_Add` _weaponlist _asusable_weapon 1))))
          (:`CastFailed`
            (bind _asconsumable_item (castclass `ConsumableItem` _itemtogive))
            (if (`BlueprintMapLibrary.Map_Contains` _consumablelist _asconsumable_item)
              (`BlueprintMapLibrary.Map_Add` _consumablelist _asconsumable_item (+ (`BlueprintMapLibrary.Map_Find` _consumablelist _asconsumable_item) 1))
              (else
                (`BlueprintMapLibrary.Map_Add` _consumablelist _asconsumable_item 1)))))
        (`/Game/Blueprints/Items/BP_ItemPickup.UsePickup` (`self.InteractObject`))
        (`/Game/UI/WB_PlayerStats.Fill Inventory` (`self.UI`) (`/Game/Blueprints/Player/BP_PlayerInventory.WeaponList` _bp_playerinventory_2) (`/Game/Blueprints/Player/BP_PlayerInventory.ConsumableList` _bp_playerinventory_2))))))

(event `EnhancedInput|/Game/ThirdPerson/Input/Actions/IA_Escape`
  (params (ActionValue :type Boolean) (ElapsedSeconds :type "Float (double-precision)") (TriggeredSeconds :type "Float (double-precision)") (InputAction :type "InputAction Object Reference" :default "/Game/ThirdPerson/Input/Actions/IA_Escape.IA_Escape"))
  (bind _returnvalue (`GameplayStatics.GetPlayerController` 0))
  (bind _ui (`self.UI`))
  (bind _bp_playerinventory (`self.BP_PlayerInventory`))
  ;[1 1 1] Escape Logic
  (:`Started`
    (if (`/Game/Blueprints/Player/BP_PlayerInventory.isOpen` _bp_playerinventory)
      (set `/Game/Blueprints/Player/BP_PlayerInventory.isOpen` false _bp_playerinventory)
      (set `PlayerController.bShowMouseCursor` false _returnvalue)
      (`WidgetBlueprintLibrary.SetInputMode_GameOnly` _returnvalue)
      (`/Game/UI/WB_PlayerStats.Close Menu` _ui)
      (else
        (set `/Game/Blueprints/Player/BP_PlayerInventory.isOpen` true _bp_playerinventory)
        (set `PlayerController.bShowMouseCursor` true _returnvalue)
        (`WidgetBlueprintLibrary.SetInputMode_GameAndUIEx` _returnvalue _ui "LockOnCapture" false)
        (`/Game/UI/WB_PlayerStats.Open Menu` _ui)))))

(event `self.ReceiveAnyDamage`
  (params (Damage :type "Float (single-precision)") (DamageType :type "DamageType Object Reference") (InstigatedBy :type "Controller Object Reference") (DamageCauser :type "Actor Object Reference"))
  ;[1 1 1] Damaged
  (`self.ReduceHealth` Damage)
  (`self.NextState` (`self.PA_MediumDamage`)))

(event `EnhancedInput|/Game/ThirdPerson/Input/Actions/IA_Move`
  (params (ActionValue :type "Vector2D Structure") (ElapsedSeconds :type "Float (double-precision)") (TriggeredSeconds :type "Float (double-precision)") (InputAction :type "InputAction Object Reference" :default "/Game/ThirdPerson/Input/Actions/IA_Move.IA_Move")))

(fn `FindLockOnTarget`
  (locals (LockOnOptions :type "Map of EnemyCharacter Object Reference to Float (double-precision)"))
  (bind _returnvalue (`WidgetLayoutLibrary.GetViewportSize`))
  (bind _lockonoptions (`local.LockOnOptions`))
  ;[1 1 1] Get Enemy List
  (bind _outactors (`GameplayStatics.GetAllActorsWithTag` "Enemy"))
  (if (> (`KismetArrayLibrary.Array_Length` _outactors) 0)
    ;[1 1 1] Reset LockOn Options
    (`BlueprintMapLibrary.Map_Clear` (`local.LockOnOptions`))
    ;[1 1 1] Populate Options List
    (for _array_element _outactors
      (bind _asenemy_character (cast `EnemyCharacter` _array_element))
      (bind _screenposition (`GameplayStatics.ProjectWorldToScreen` (`GameplayStatics.GetPlayerController` 0) (`self.K2_GetActorLocation` _array_element)))
      (bind _returnvalue_2 (`self.IsOnScreen` _returnvalue _screenposition))
      (if _returnvalue_2
        (`BlueprintMapLibrary.Map_Add` (`local.LockOnOptions`) _asenemy_character (`KismetMathLibrary.Distance2D` (/ _returnvalue 2.0) _screenposition))))
    ;[1 1 1] Find Closest Target To Lock On
    (bind _keys (`BlueprintMapLibrary.Map_Keys` (`local.LockOnOptions`)))
    (set `self.LockOnTarget` (`|GetArrayItem` _keys))
    (for _array_element_2 _keys
      (if (< (`BlueprintMapLibrary.Map_Find` _lockonoptions _array_element_2) (`BlueprintMapLibrary.Map_Find` _lockonoptions (`self.LockOnTarget`)))
        (set `self.LockOnTarget` _array_element_2)))
    (set `self.bUseControllerRotationYaw` true)))

(fn `InitializeActionList`
  (bind _statelist (`self.StateList`))
  (`BlueprintMapLibrary.Map_Add` _statelist "NewEnumerator0" (`self.PA_Base`))
  (`BlueprintMapLibrary.Map_Add` _statelist "NewEnumerator1" (`self.PA_Dodge`)))

(fn `NextState`
  (params (NewState :type "/Game/Blueprints/Player/BP_PlayerAction Object Reference"))
  (returns (Success :type Boolean))
  (if (<= (`/Game/Blueprints/Player/BP_PlayerAction.StaminaCost` NewState) (`CharacterStats.currentStamina` (`self.stats`)))
    (`self.UseStamina` (`/Game/Blueprints/Player/BP_PlayerAction.StaminaCost` NewState))
    (bind _output_get (set `self.CurrentState` NewState))
    (`/Game/Blueprints/Player/BP_PlayerAction.Use Action` _output_get)
    (return true)
    (else
      (return false))))

(fn `ReduceHealth`
  (params (Damage :type "Float (double-precision)"))
  (returns (`New Health` :type "Float (double-precision)"))
  (bind _stats (`self.stats`))
  (bind _output_get (set `CharacterStats.currentHealth` (`KismetMathLibrary.FClamp` (- (`CharacterStats.currentHealth` _stats) Damage) 0.0 (`CharacterStats.maximumHealth` _stats)) _stats))
  (return _output_get))

(fn `UpdateCanAct`
  (if (and (== (`self.CurrentState`) (`self.PA_Base`)) (not (`/Game/Blueprints/Player/BP_PlayerInventory.isOpen` (`self.BP_PlayerInventory`))))
    (set `self.CanAct` true)
    (else
      (set `self.CanAct` false))))

(fn `UpdateStamina`
  (params (DeltaTime :type "Float (double-precision)"))
  (returns (NewStamina :type "Float (double-precision)"))
  (bind _stats (`self.stats`))
  (bind _currentstamina (`CharacterStats.currentStamina` _stats))
  (bind _maximumstamina (`CharacterStats.maximumStamina` _stats))
  (if (< _currentstamina _maximumstamina)
    (bind _output_get (set `CharacterStats.currentStamina` (`KismetMathLibrary.FClamp` (+ _currentstamina (* (`CharacterStats.staminaPerSecond` _stats) DeltaTime)) 0.0 _maximumstamina) _stats))
    (return _output_get)))

(fn `UserConstructionScript`)

(fn `UseStamina`
  (params (Cost :type "Float (double-precision)"))
  (returns (NewStamina :type "Float (double-precision)"))
  (bind _stats (`self.stats`))
  (bind _output_get (set `CharacterStats.currentStamina` (`KismetMathLibrary.FClamp` (- (`CharacterStats.currentStamina` _stats) Cost) 0.0 (`CharacterStats.maximumStamina` _stats)) _stats))
  (return _output_get))