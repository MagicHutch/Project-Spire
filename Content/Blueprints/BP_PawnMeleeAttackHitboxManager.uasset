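; Manager for pawn melee hitboxes that turns overlaps into damage on the actors hit.
; Registered hitboxes bind overlap events and map to a damage value and an active flag, which also drives visibility.
; Active-hitbox overlaps queue damageable actors, players only via their CurrentDamageHitbox, and Tick damages then clears the queue.
; An ActorsToIgnore list tracks the owner and damaged actors until overlap ends, but is never checked before damaging.
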(event `self.ReceiveBeginPlay`
  (`KismetArrayLibrary.Array_Add` (`self.ActorsToIgnore`) (`self.GetOwner`)))

(event `self.ReceiveTick`
  (params (DeltaSeconds :type "Float (single-precision)"))
  (`self.TickProcessHitActors`))

(event `ConfigureBindings`
  (params (CompToBind :type "PrimitiveComponent Object Reference"))
  (add `PrimitiveComponent.OnComponentBeginOverlap` CompToBind (delegate `OnComponentBeginOverlap_Event`))
  (add `PrimitiveComponent.OnComponentEndOverlap` CompToBind (delegate `OnComponentEndOverlap_Event`)))

(event `OnComponentBeginOverlap_Event`
  (params (OverlappedComponent :type "PrimitiveComponent Object Reference") (OtherActor :type "Actor Object Reference") (OtherComp :type "PrimitiveComponent Object Reference") (OtherBodyIndex :type Integer) (bFromSweep :type Boolean) (SweepResult :type "HitResult Structure (by ref)"))
  (`self.ProcessBeginOverlap` OverlappedComponent OtherActor OtherComp))

(event `OnComponentEndOverlap_Event`
  (params (OverlappedComponent :type "PrimitiveComponent Object Reference") (OtherActor :type "Actor Object Reference") (OtherComp :type "PrimitiveComponent Object Reference") (OtherBodyIndex :type Integer))
  (`self.ProcessEndOverlap` OtherActor))

(fn `AddHitboxToComponent`
  (params (ComponentToAdd :type "PrimitiveComponent Object Reference") (AttachedDamageValue :type "Float (double-precision)"))
  (`|ExecutionSequence`
    (:`then_0`
      (`BlueprintMapLibrary.Map_Add` (`self.HitboxMap`) (`local.ComponentToAdd`)))
    (:`then_1`
      (`BlueprintMapLibrary.Map_Add` (`self.DamageMap`) (`local.ComponentToAdd`) (`local.AttachedDamageValue`)))
    (:`then_2`
      (`self.ConfigureBindings` (`local.ComponentToAdd`)))))

(fn `ProcessBeginOverlap`
  (params (InOverlappedComponent :type "PrimitiveComponent Object Reference") (InOtherActor :type "Actor Object Reference") (InOtherComp :type "PrimitiveComponent Object Reference"))
  (if (`BlueprintMapLibrary.Map_Find` (`self.HitboxMap`) (`local.InOverlappedComponent`))
    (if (`Actor.bCanBeDamaged` (`local.InOtherActor`))
      (bind _asbp_player_v3 (cast `/Game/Blueprints/Player/BP_PlayerV3` (`local.InOtherActor`))
        (:`then`
          (if (== (`/Game/Blueprints/Player/BP_PlayerV3.currentDamageHitbox` _asbp_player_v3) (`local.InOtherComp`))
            (`BlueprintMapLibrary.Map_Add` (`self.HitActors`) (`local.InOtherActor`) (`local.InOverlappedComponent`) :!label _label)))
        (:`CastFailed`
          (goto _label))))))

(fn `ProcessEndOverlap`
  (params (InOtherActor :type "Actor Object Reference"))
  (if (`KismetArrayLibrary.Array_Contains` (`self.ActorsToIgnore`) (`local.InOtherActor`))
    (`KismetArrayLibrary.Array_RemoveItem` (`self.ActorsToIgnore`) (`local.InOtherActor`))))

(fn `SetHitboxIsActivated`
  (params (HitboxToToggle :type "PrimitiveComponent Object Reference") (isActivated :type Boolean))
  (`BlueprintMapLibrary.Map_Add` (`self.HitboxMap`) HitboxToToggle isActivated)
  (`SceneComponent.SetVisibility` HitboxToToggle isActivated false))

(fn `TickProcessHitActors`
  (bind _keys (`BlueprintMapLibrary.Map_Keys` (`self.HitActors`)))
  (for _array_element _keys
    (`GameplayStatics.ApplyDamage` _array_element (`BlueprintMapLibrary.Map_Find` (`self.DamageMap`) (`BlueprintMapLibrary.Map_Find` (`self.HitActors`) _array_element)))
    (`KismetArrayLibrary.Array_Add` (`self.ActorsToIgnore`) _array_element))
  (`BlueprintMapLibrary.Map_Clear` (`self.HitActors`)))