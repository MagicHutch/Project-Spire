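; Gaol Warden boss enemy whose action components serve as named states, with those flagged as attacks pooled for random selection.
; Spawns a club, staff and guard sword, shares the weapons with attack actions, and pins them to bones each tick.
; Below half health an extra arm appears, looping sword swings; below 15%, Cover becomes flagged as an attack.
; Head hits during Overhead Smash deal bonus damage, release held weapons and trigger stagger.
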(event `self.ReceiveBeginPlay`
  (bind _arm (`self.Arm`))
  (`parent.ReceiveBeginPlay`)
  (`ActorComponent.SetComponentTickEnabled` _arm false)
  (`SceneComponent.SetVisibility` _arm false false)
  (for _array_element (`self.K2_GetComponentsByClass` "/Game/Blueprints/Enemies/BP_EnemyAction.BP_EnemyAction_C")
    (if (`EnemyAction.isAttackAction` _array_element)
      (`KismetArrayLibrary.Array_Add` (`self.AttackActions`) _array_element)))
  (bind _returnvalue (`|SpawnActorFromClass` "/Game/Blueprints/Items/Weapons/NewWeapons/BP_WardenClub.BP_WardenClub_C" (`KismetMathLibrary.MakeTransform` (0.0 0.0 0.0)) "Undefined" "MultiplyWithRoot" null null))
  (bind _output_get (set `self.WardenClubReference` _returnvalue))
  (bind _output_get_2 (set `/Game/Blueprints/Bosses/GaolWarden/Actions/EA_GaolWarden_ClubSmash.OwnerClubReference` _output_get (`self.EA_GaolWarden_ClubSmash`)))
  (bind _output_get_3 (set `/Game/Blueprints/Bosses/GaolWarden/Actions/EA_GaolWarden_JumpSmash.OwnerClubReference` _output_get_2 (`self.EA_GaolWarden_JumpSmash`)))
  (bind _output_get_4 (set `/Game/Blueprints/Bosses/GaolWarden/Actions/EA_GaolWarden_FrontArc.OwnerClubReference` _output_get_3 (`self.EA_GaolWarden_FrontArc`)))
  (set `/Game/Blueprints/Bosses/GaolWarden/Actions/EA_GaolWarden_OverheadSmash.OwnerClubReference` _output_get_4 (`self.EA_GaolWarden_OverheadSmash`))
  (bind _returnvalue_2 (`|SpawnActorFromClass` "/Game/Blueprints/Items/Weapons/NewWeapons/BP_WardenStaff.BP_WardenStaff_C" (`KismetMathLibrary.MakeTransform` (0.0 0.0 0.0)) "Undefined" "MultiplyWithRoot" null null))
  (bind _output_get_5 (set `self.WardenStaffReference` _returnvalue_2))
  (bind _output_get_6 (set `/Game/Blueprints/Bosses/GaolWarden/Actions/EA_GaolWarden_FrontArc.OwnerStaffReference` _output_get_5 (`self.EA_GaolWarden_FrontArc`)))
  (bind _output_get_7 (set `/Game/Blueprints/Bosses/GaolWarden/Actions/EA_GaolWarden_ThreeStab.OwnerStaffReference` _output_get_6 (`self.EA_GaolWarden_ThreeStab`)))
  (set `/Game/Blueprints/Bosses/GaolWarden/Actions/EA_GaolWarden_OverheadSmash.OwnerStaffReference` _output_get_7 (`self.EA_GaolWarden_OverheadSmash`))
  (set `/Game/Blueprints/Bosses/GaolWarden/Actions/EA_GaolWarden_HighClap.ClapWaveRefernce` (`self.ClapWave`) (`self.EA_GaolWarden_HighClap`))
  (bind _returnvalue_3 (`|SpawnActorFromClass` "/Game/Blueprints/Items/Weapons/NewWeapons/BP_FugitiveShortSword.BP_FugitiveShortSword_C" (`KismetMathLibrary.MakeTransform` (0.0 0.0 0.0)) "Undefined" "MultiplyWithRoot" null null))
  (bind _output_get_8 (set `self.GuardSword` _returnvalue_3))
  (set `/Game/Blueprints/Items/Weapons/NewWeapons/BP_UsableWeapon.ActorClassesToIgnore` (`|MakeArray` "/Script/MyProject.EnemyCharacter" :!type "Actor Class Reference") _output_get_8)
  (`SceneComponent.SetVisibility` (`/Game/Blueprints/Items/Weapons/NewWeapons/BP_UsableWeapon.StaticMesh` _output_get_8) false false))

(event `self.ReceiveTick`
  (params (DeltaSeconds :type "Float (single-precision)"))
  (bind _stats (`self.stats`))
  (`parent.ReceiveTick` DeltaSeconds)
  (`self.UpdateEquipment`)
  (`self.Calculate Advantage`)
  (`self.EnableArm`)
  (if (and (not (`EnemyAction.isAttackAction` (`self.EA_GaolWarden_Cover`))) (< (/ (`CharacterStats.currentHealth` _stats) (`CharacterStats.maximumHealth` _stats)) 0.15))
    (set `EnemyAction.isAttackAction` true (`self.EA_GaolWarden_Cover`))))

(event `self.PopulateActionList`
  (`BlueprintMapLibrary.Map_Add` (`self.ActionList`) "IDLE" (`self.EA_GaolWarden_Idle`))
  (`BlueprintMapLibrary.Map_Add` (`self.ActionList`) "CHASE" (`self.EA_GaolWarden_Chase`))
  (`BlueprintMapLibrary.Map_Add` (`self.ActionList`) "CLUBSMASH" (`self.EA_GaolWarden_ClubSmash`))
  (`BlueprintMapLibrary.Map_Add` (`self.ActionList`) "TWOSTOMP" (`self.EA_GaolWarden_TwoStomp`))
  (`BlueprintMapLibrary.Map_Add` (`self.ActionList`) "JUMPSMASH" (`self.EA_GaolWarden_JumpSmash`))
  (`BlueprintMapLibrary.Map_Add` (`self.ActionList`) "COVER" (`self.EA_GaolWarden_Cover`))
  (`BlueprintMapLibrary.Map_Add` (`self.ActionList`) "FRONTARC" (`self.EA_GaolWarden_FrontArc`))
  (`BlueprintMapLibrary.Map_Add` (`self.ActionList`) "THREESTAB" (`self.EA_GaolWarden_ThreeStab`))
  (`BlueprintMapLibrary.Map_Add` (`self.ActionList`) "OVERHEAD" (`self.EA_GaolWarden_OverheadSmash`))
  (`BlueprintMapLibrary.Map_Add` (`self.ActionList`) "STAGGER" (`self.EA_GaolWarden_Stagger`))
  (`BlueprintMapLibrary.Map_Add` (`self.ActionList`) "HIGHCLAP" (`self.EA_GaolWarden_HighClap`))
  (`BlueprintMapLibrary.Map_Add` (`self.ActionList`) "PUNCHTOKICK" (`self.EA_GaolWarden_PunchToKick`))
  (`BlueprintMapLibrary.Map_Add` (`self.ActionList`) "THREESMASH" (`self.EA_GaolWarden_ThreeSmash`))
  (`BlueprintMapLibrary.Map_Add` (`self.ActionList`) "SPINNINGKICK" (`self.EA_GaolWarden_SpinningKick`))
  (`BlueprintMapLibrary.Map_Add` (`self.ActionList`) "LUNGECLAP" (`self.EA_GaolWarden_LungeClap`)))

(event `self.KillEntity`
  (`self.K2_DestroyActor` (`self.WardenStaffReference`))
  (`self.K2_DestroyActor` (`self.WardenClubReference`))
  (`self.K2_DestroyActor` (`self.GuardArm`))
  (`self.K2_DestroyActor` (`self.GuardSword`))
  (bind _asbp_player_v3 (cast `/Game/Blueprints/Player/BP_PlayerV3` (`self.player`)))
  (`/Game/Blueprints/Player/BP_PlayerV3.RemoveBossHealthBar` _asbp_player_v3 self))

(event `GuardArmSwing`
  (bind _guardsword (`self.GuardSword`))
  (`KismetSystemLibrary.PrintString` "Hello")
  (`|PlayMontage` (`self.Arm`) "/Game/Characters/Enemies/GaolGuardArm/Animations/Assets/AM_SwingSequence1.AM_SwingSequence1"
    (:`OnCompleted`
      (`self.GuardArmSwing`))
    (:`OnNotifyBegin`
      (`UsableWeapon.ActivateAttack` _guardsword))
    (:`OnNotifyEnd`
      (`UsableWeapon.DeactivateAttack` _guardsword))))

(event `self.SpecialHitboxLogic`
  (params (Damage :type "Float (double-precision)"))
  (bind _stats (`self.stats`))
  (bind _overlappingactors (`PrimitiveComponent.GetOverlappingActors` (`self.HeadHitbox`) "/Game/Blueprints/Items/Weapons/NewWeapons/BP_UsableWeapon.BP_UsableWeapon_C"))
  (if (and (> (`KismetArrayLibrary.Array_Length` _overlappingactors) 0) (== (`self.currentState`) (`self.EA_GaolWarden_OverheadSmash`)))
    (for _array_element _overlappingactors
      (bind _asbp_usable_weapon (cast `/Game/Blueprints/Items/Weapons/NewWeapons/BP_UsableWeapon` _array_element))
      (if (not (or (`KismetArrayLibrary.Array_Contains` (`/Game/Blueprints/Items/Weapons/NewWeapons/BP_UsableWeapon.ActorClassesToIgnore` _asbp_usable_weapon) "/Game/Blueprints/Enemies/BP_EnemyCharacter.BP_EnemyCharacter_C") (`KismetArrayLibrary.Array_Contains` (`/Game/Blueprints/Items/Weapons/NewWeapons/BP_UsableWeapon.ActorClassesToIgnore` _asbp_usable_weapon) "/Script/MyProject.EnemyCharacter")))
        (set `CharacterStats.currentHealth` (`KismetMathLibrary.FClamp` (- (`CharacterStats.currentHealth` _stats) (* Damage 15.0)) 0.0 (`CharacterStats.maximumHealth` _stats)) _stats)
        (`KismetSystemLibrary.PrintString` "Head Hit!")
        (set `self.isHoldingWeapons` false)
        (`/Game/Blueprints/Enemies/BP_EnemyAction.SwitchToState` (`self.EA_GaolWarden_Idle`) "STAGGER")
        (break)))))

(event `self.ClapWave.OnComponentBeginOverlap`
  (params (OverlappedComponent :type "PrimitiveComponent Object Reference") (OtherActor :type "Actor Object Reference") (OtherComp :type "PrimitiveComponent Object Reference") (OtherBodyIndex :type Integer) (bFromSweep :type Boolean) (SweepResult :type "HitResult Structure (by ref)"))
  (if (== (`GameplayStatics.GetObjectClass` OtherActor) "/Game/Blueprints/Player/BP_PlayerV3.BP_PlayerV3_C")
    (`GameplayStatics.ApplyDamage` OtherActor 30.0)))

(fn `EnableArm`
  (bind _stats (`self.stats`))
  (bind _arm (`self.Arm`))
  (if (and (not (`SceneComponent.IsVisible` (`self.Arm`))) (< (/ (`CharacterStats.currentHealth` _stats) (`CharacterStats.maximumHealth` _stats)) 0.5))
    (`ActorComponent.SetComponentTickEnabled` _arm true)
    (`SceneComponent.SetVisibility` _arm true false)
    (`self.GuardArmSwing`)
    (`SceneComponent.SetVisibility` (`/Game/Blueprints/Items/Weapons/NewWeapons/BP_UsableWeapon.StaticMesh` (`self.GuardSword`)) true false))
  (return))

(fn `PickRandomAction`
  (returns (`return state` :type "EnemyAction Object Reference"))
  (return (`KismetArrayLibrary.Array_Random` (`self.AttackActions`))))

(fn `UpdateEquipment`
  (bind _mesh (`self.Mesh`))
  (bind _arm (`self.Arm`))
  (bind (_returnvalue_location _returnvalue_rotation) (`KismetMathLibrary.BreakTransform` (`SkinnedMeshComponent.GetBoneTransform` _mesh "hand_r" "RTS_World")))
  (bind (_returnvalue_location_2 _returnvalue_rotation_2) (`KismetMathLibrary.BreakTransform` (`SkinnedMeshComponent.GetBoneTransform` _mesh "hand_l" "RTS_World")))
  (bind (_returnvalue_location_3 _returnvalue_rotation_3) (`KismetMathLibrary.BreakTransform` (`SkinnedMeshComponent.GetBoneTransform` _arm "Bone_002" "RTS_World")))
  (`SceneComponent.K2_SetWorldRotation` _arm (`KismetMathLibrary.MakeRotator` 0.0 -90.0 (+ (.yaw (.rotation (`SkinnedMeshComponent.GetBoneTransform` (`self.Mesh`) "spine01" "RTS_World"))) 270.0)) false false)
  (`self.K2_SetActorLocationAndRotation` (`self.GuardSword`) (+ _returnvalue_location_3 (* (`KismetMathLibrary.GetRightVector` _returnvalue_rotation_3) -20.0)) _returnvalue_rotation_3 true false)
  (if (`self.isHoldingWeapons`)
    (`self.K2_SetActorLocationAndRotation` (`self.WardenClubReference`) (+ _returnvalue_location (* (`KismetMathLibrary.GetRightVector` _returnvalue_rotation) -20.0)) _returnvalue_rotation true false)
    (`self.K2_SetActorLocationAndRotation` (`self.WardenStaffReference`) (+ _returnvalue_location_2 (* (`KismetMathLibrary.GetRightVector` _returnvalue_rotation_2) -20.0)) _returnvalue_rotation_2 true false)
    (return)))

(fn `UserConstructionScript`
  (`parent.UserConstructionScript`)
  (bind _output_get (set `self.entryState` (`self.EA_GaolWarden_Idle`)))
  (set `self.currentState` _output_get)
  (`self.PopulateActionList`))