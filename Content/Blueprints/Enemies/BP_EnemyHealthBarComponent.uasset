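; Enemy component that shows a floating health readout over a damaged BP_EnemyCharacter when the player is nearby.
; Every Tick it casts its owner and checks that the offset display position is within range of the player pawn and that current health is below maximum.
; The readout is red current / maximum text drawn with DrawDebugString rather than a bar or UMG widget.
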(event `self.ReceiveTick`
  (params (DeltaSeconds :type "Float (single-precision)"))
  (bind _returnvalue (`self.GetOwner`))
  (bind _returnvalue_2 (+ (`Actor.K2_GetActorLocation` _returnvalue) (`self.DisplayPositionAdjust`)))
  (bind _asbp_enemy_character (cast `/Game/Blueprints/Enemies/BP_EnemyCharacter` _returnvalue))
  (bind _stats (`EnemyCharacter.stats` _asbp_enemy_character))
  (bind _currenthealth (`CharacterStats.currentHealth` _stats))
  (bind _maximumhealth (`CharacterStats.maximumHealth` _stats))
  (if (and (< (`KismetMathLibrary.Vector_Distance` _returnvalue_2 (`Actor.K2_GetActorLocation` (`GameplayStatics.GetPlayerPawn` 0))) 500.0) (< _currenthealth _maximumhealth))
    (`KismetSystemLibrary.DrawDebugString` _returnvalue_2 (`KismetTextLibrary.Conv_TextToString` (`|FormatText` "{0} / {1}" _currenthealth _maximumhealth)) null (struct :`R` 1.0 :`A` 1.0))))