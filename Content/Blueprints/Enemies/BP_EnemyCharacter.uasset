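; Base enemy character with stats, aggro detection, tethering and death handling, leaving empty hooks for special hitboxes, cleanup and boss aggro.
; It enters its entry state on spawn, then each tick updates health advantage over the player, tether limits and state-gated stamina regen.
; Damage applies damage-circle boons and feeds player Will.
; Player kills award Or and record the level ID in GlobalTempData, so the enemy is removed on later loads.
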(event `self.ReceiveBeginPlay`
  (bind _asglobal_temp_data (cast `GlobalTempData` (`GameplayStatics.GetGameInstance`)))
  (bind _output_get (set `self.GlobalTempData` _asglobal_temp_data))
  (`self.CheckShouldRemoveEntityOnStart`)
  (`KismetArrayLibrary.Array_Add` (`GlobalTempData.enemiesInScene` _output_get) self)
  (bind _asbp_player_v3 (cast `/Game/Blueprints/Player/BP_PlayerV3` (`GameplayStatics.GetPlayerPawn` 0)))
  (set `self.player` _asbp_player_v3)
  (set `self.tetherPosition` (`self.K2_GetActorLocation`))
  (`self.NextState` (`self.entryState`)))

(event `self.ReceiveTick`
  (params (DeltaSeconds :type "Float (single-precision)"))
  (bind _stats (`self.stats`))
  ;[1 1 1] Tick
  (`self.Calculate Advantage`)
  (`self.ManageTether`)
  (if (`EnemyAction.canRegainStamina` (`self.currentState`))
    (set `CharacterStats.currentStamina` (`KismetMathLibrary.FClamp` (+ (`CharacterStats.currentStamina` _stats) (* (`CharacterStats.staminaPerSecond` _stats) DeltaSeconds)) 0.0 (`CharacterStats.maximumStamina` _stats)) _stats)))

(event `self.ReceiveAnyDamage`
  (params (Damage :type "Float (single-precision)") (DamageType :type "DamageType Object Reference") (InstigatedBy :type "Controller Object Reference") (DamageCauser :type "Actor Object Reference"))
  ;[1 1 1] Take Damage
  (bind _finaldamage (`self.CalculateDamageHealthLoss` Damage))
  (`self.SpecialHitboxLogic` _finaldamage)
  (bind _asbp_player_v3 (cast `/Game/Blueprints/Player/BP_PlayerV3` (`GameplayStatics.GetPlayerPawn` 0)))
  (`/Game/Blueprints/Player/BP_PlayerV3.IncreaseWill` _asbp_player_v3 (* (/ _finaldamage (`CharacterStats.maximumHealth` (`self.stats`))) (/ (`CharacterStats.maximumHealth` (`self.stats`)) (`CharacterStats.maximumHealth` (`PlayerControllerV2.stats` _asbp_player_v3)))))
  (if (<= _finaldamage 0.0)
    (set `/Game/Blueprints/Player/BP_PlayerV3.LockOnTarget` null _asbp_player_v3)
    (`self.KillEntity` true)))

(event `KillEntity`
  (params (isFirstKill :type Boolean))
  (bind _player (`self.player`))
  (`self.KillCleanupEvent`)
  (if isFirstKill
    (set `PlayerControllerV2.orCount` (+ (`PlayerControllerV2.orCount` _player) (`self.orValue`)) _player)
    (`self.UpdateLevelData`))
  (`KismetArrayLibrary.Array_RemoveItem` (`GlobalTempData.enemiesInScene` (`self.GlobalTempData`)) self)
  (`self.K2_DestroyActor`))

(event `KillCleanupEvent`)

(event `PopulateActionList`)

(event `SpecialHitboxLogic`
  (params (Damage :type "Float (double-precision)")))

(event `TetherLimitReached`
  (`KismetSystemLibrary.PrintString` "Tethered"))

(event `BossAggroTrigger`)

(event `self.CapsuleComponent.OnComponentHit`
  (params (HitComponent :type "PrimitiveComponent Object Reference") (OtherActor :type "Actor Object Reference") (OtherComp :type "PrimitiveComponent Object Reference") (NormalImpulse :type "Vector Structure") (Hit :type "HitResult Structure (by ref)"))
  (cast `/Game/Blueprints/IntersectionObjects/BP_TestIntersectionObject` OtherActor)
  (`KismetSystemLibrary.PrintString` "I'm hit!"))

(fn `Calculate Advantage`
  (returns (NewAdvantage :type "Float (double-precision)"))
  (bind _stats (`self.stats`))
  (bind _asbp_player_v3 (cast `/Game/Blueprints/Player/BP_PlayerV3` (`self.player`)))
  (bind _stats_2 (`PlayerControllerV2.stats` _asbp_player_v3))
  (bind _output_get (set `self.advantage` (- (/ (`CharacterStats.currentHealth` _stats) (`CharacterStats.maximumHealth` _stats)) (/ (`CharacterStats.currentHealth` _stats_2) (`CharacterStats.maximumHealth` _stats_2)))))
  (return _output_get))

(fn `CalculateDamageHealthLoss`
  (params (rawDamage :type "Float (double-precision)"))
  (returns (finalDamage :type "Float (double-precision)"))
  (bind _stats (`self.stats`))
  (bind _stats_2 (`self.stats`))
  (bind _returnvalue (`GameplayStatics.GetActorOfClass` "/Game/Blueprints/Items/Boons_and_Strains/Boons/BP_Boon_DamageCircle.BP_Boon_DamageCircle_C"))
  (if (`KismetSystemLibrary.IsValid` _returnvalue)
    (if (`KismetArrayLibrary.Array_Contains` (`/Game/Blueprints/Items/Boons_and_Strains/Boons/BP_Boon_DamageCircle.containedActors` _returnvalue) self)
      (bind _output_get (set `CharacterStats.currentHealth` (`KismetMathLibrary.FClamp` (- (`CharacterStats.currentHealth` _stats_2) (* (`local.rawDamage`) (`/Game/Blueprints/Items/Boons_and_Strains/Boons/BP_Boon_DamageCircle.damageBoost` _returnvalue))) 0.0 (`CharacterStats.maximumHealth` _stats_2)) _stats_2))
      (return _output_get)
      (else
        _)))
  (bind _output_get_2 (set `CharacterStats.currentHealth` (`KismetMathLibrary.FClamp` (- (`CharacterStats.currentHealth` _stats) (`local.rawDamage`)) 0.0 (`CharacterStats.maximumHealth` _stats)) _stats))
  (return _output_get_2))

(fn `CheckPlayerInFieldOfView`
  (params (inputFOV :type "Float (double-precision)"))
  (returns (isInFov :type Boolean))
  (bind (_returnvalue_x _returnvalue_y _returnvalue_z) (`KismetMathLibrary.BreakVector` (`self.K2_GetActorLocation`)))
  (bind _player (`self.player`))
  (bind _returnvalue (`self.AngleBetweenVectors` (`KismetMathLibrary.GetForwardVector` (`self.K2_GetActorRotation`)) (- (`self.K2_GetActorLocation` _player) (`self.K2_GetActorLocation`))))
  (if (and (<= _returnvalue inputFOV) (< (`self.GetDistanceTo` _player) 1000.0))
    (bind _outhit (`KismetSystemLibrary.LineTraceSingleForObjects` (`KismetMathLibrary.MakeVector` _returnvalue_x _returnvalue_y (+ _returnvalue_z (`CapsuleComponent.GetScaledCapsuleHalfHeight` (`self.CapsuleComponent`)))) (`self.K2_GetActorLocation` (`self.player`)) (`|MakeArray` "ObjectTypeQuery1" "ObjectTypeQuery3" :!type "EObjectTypeQuery Enum")))
    (if (== (`self.player`) (`.HitActor` (`GameplayStatics.BreakHitResult` _outhit)))
      (return true)
      (else
        (return false)))
    (else
      (return false))))

(fn `CheckPlayerSelfElevationDifference`
  (returns (verticalDifference :type "Float (double-precision)"))
  (bind (_returnvalue_x _returnvalue_y _returnvalue_z) (`KismetMathLibrary.BreakVector` (`self.K2_GetActorLocation`)))
  (bind (_returnvalue_x_2 _returnvalue_y_2 _returnvalue_z_2) (`KismetMathLibrary.BreakVector` (`self.K2_GetActorLocation` (`self.player`))))
  (return (`KismetMathLibrary.VSize` (- (`KismetMathLibrary.MakeVector` 0.0 0.0 _returnvalue_z) (`KismetMathLibrary.MakeVector` 0.0 0.0 _returnvalue_z_2)))))

(fn `CheckPlayerWithinDistance`
  (params (distance :type "Float (double-precision)"))
  (returns (withinDistance :type Boolean))
  (return (<= (`self.GetDistanceTo` (`self.player`)) distance)))

(fn `CheckSetAggroTrue`
  (params (maxDistanceDifference :type "Float (double-precision)") (maxElevationDifference :type "Float (double-precision)") (fieldOfView :type "Float (double-precision)"))
  (returns (isAggro :type Boolean))
  (bind (_returnvalue_x _returnvalue_y _returnvalue_z) (`KismetMathLibrary.BreakVector` (`self.K2_GetActorLocation`)))
  (bind _isinfov (`self.CheckPlayerInFieldOfView` (`local.fieldOfView`)))
  (bind _withindistance (`self.CheckPlayerWithinDistance` (`local.maxDistanceDifference`)))
  (bind _verticaldifference (`self.CheckPlayerSelfElevationDifference`))
  (bind _returnvalue (< _verticaldifference (`local.maxElevationDifference`)))
  (if (or (and _isinfov _returnvalue) (and _returnvalue _withindistance))
    (bind _outhit (`KismetSystemLibrary.LineTraceSingleForObjects` (`KismetMathLibrary.MakeVector` _returnvalue_x _returnvalue_y (+ _returnvalue_z (`CapsuleComponent.GetScaledCapsuleHalfHeight` (`self.CapsuleComponent`)))) (`self.K2_GetActorLocation` (`self.player`)) (`|MakeArray` "ObjectTypeQuery1" "ObjectTypeQuery3" :!type "EObjectTypeQuery Enum")))
    (if (== (`self.player`) (`.HitActor` (`GameplayStatics.BreakHitResult` _outhit)))
      (set `self.isAggro` true)
      (return true)
      (else
        (set `self.isAggro` false)
        (return false)))
    (else
      (set `self.isAggro` false)
      (return false))))

(fn `CheckShouldRemoveEntityOnStart`
  (if (`KismetStringLibrary.NotEqual_StrStr` (`self.enemyLevelID`))
    (if (== (`BlueprintMapLibrary.Map_Find` (`GlobalTempData.levelObjectStateData` (`self.GlobalTempData`)) (`self.enemyLevelID`)) 1)
      (`self.KillEntity` false))))

(fn `CreateDamageDisplay`
  (params (damageToDisplay :type "Float (double-precision)"))
  (bind (_returnvalue_x _returnvalue_y _returnvalue_z) (`KismetMathLibrary.BreakVector` (`self.K2_GetActorLocation`)))
  (`KismetSystemLibrary.DrawDebugString` (`KismetMathLibrary.MakeVector` _returnvalue_x _returnvalue_y (+ _returnvalue_z (+ (`CapsuleComponent.GetScaledCapsuleHalfHeight` (`self.CapsuleComponent`)) 30.0))) (`KismetStringLibrary.Conv_DoubleToString` damageToDisplay) null (struct :`R` 1.0 :`B` 0.075054 :`A` 1.0) 5.0))

(fn `CreateHealthBar`
  (if (not (`KismetSystemLibrary.IsValid` (`self.HealthBar`)))
    (bind _returnvalue (`|CreateWidget` "/Game/UI/NewUI/SubWidgets/WB_EnemyHealthBar.WB_EnemyHealthBar_C"))
    (bind _output_get (set `self.HealthBar` _returnvalue))
    (set `/Game/UI/NewUI/SubWidgets/WB_EnemyHealthBar.AssociatedEnemy` self _output_get)))

(fn `ManageTether`
  (bind (_returnvalue_x _returnvalue_y _returnvalue_z) (`KismetMathLibrary.BreakVector` (`self.K2_GetActorLocation`)))
  (bind (_returnvalue_x_2 _returnvalue_y_2) (`KismetMathLibrary.BreakVector` (`self.K2_GetActorLocation`)))
  (bind (_tetherposition_x _tetherposition_y _tetherposition_z) (`KismetMathLibrary.BreakVector` (`self.tetherPosition`)))
  (bind (_tetherposition_x_2 _tetherposition_y_2) (`KismetMathLibrary.BreakVector` (`self.tetherPosition`)))
  (bind _horizontaltether (`self.horizontalTether`))
  (bind _verticaltether (`self.verticalTether`))
  (if (`self.isAggro`)
    (if (and (> (`KismetMathLibrary.Vector_Distance` (`KismetMathLibrary.MakeVector` _returnvalue_x_2 _returnvalue_y_2) (`KismetMathLibrary.MakeVector` _tetherposition_x_2 _tetherposition_y_2)) _horizontaltether) (> _horizontaltether 0.0))
      (`self.TetherLimitReached`)
      (elif (and (> (`KismetMathLibrary.Abs` (- _returnvalue_z _tetherposition_z)) _verticaltether) (> _verticaltether 0.0))
        (`self.TetherLimitReached`)))))

(fn `SetPlayerReference`
  (if true
    _))

(fn `ToggleAggro`
  (params (isAggro :type Boolean))
  (returns (newAgrroValue :type Boolean))
  (bind _output_get (set `self.isAggro` isAggro))
  (return _output_get))

(fn `UpdateHealthBar`
  (`UserWidget.SetPositionInViewport` (`self.HealthBar`) (`GameplayStatics.ProjectWorldToScreen` (`GameplayStatics.GetPlayerController` 0) (`self.K2_GetActorLocation`)) true))

(fn `UpdateLevelData`
  (if (`KismetStringLibrary.NotEqual_StrStr` (`self.enemyLevelID`))
    (`BlueprintMapLibrary.Map_Add` (`GlobalTempData.levelObjectStateData` (`self.GlobalTempData`)) (`self.enemyLevelID`) 1)))

(fn `UserConstructionScript`)

(fn `UseStamina`
  (params (`Stamina Amount` :type "Float (double-precision)"))
  (returns (`New Stamina` :type "Float (double-precision)"))
  (bind _stats (`self.stats`))
  (bind _output_get (set `CharacterStats.currentStamina` (`KismetMathLibrary.FClamp` (- (`CharacterStats.currentStamina` _stats) `Stamina Amount`) 0.0 (`CharacterStats.maximumStamina` _stats)) _stats))
  (return _output_get))