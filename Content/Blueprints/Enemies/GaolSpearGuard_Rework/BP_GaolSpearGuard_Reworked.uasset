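; Reworked gaol spear guard enemy that runs on an action-state list of idle, chase and swing-stumble, starting in idle.
; BeginPlay spawns a separate spear actor owned by the guard and passes its reference to the swing-stumble action.
; Instead of attaching the spear, Tick moves it with sweep to a hand-tuned offset from a mesh bone, matching that bone's rotation.
; Kill cleanup destroys the spear.
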(event `self.ReceiveBeginPlay`
  (`parent.ReceiveBeginPlay`)
  (bind _returnvalue (`|SpawnActorFromClass` "/Game/Blueprints/Items/Weapons/NewWeapons/BP_GuardSpear.BP_GuardSpear_C" (`KismetMathLibrary.MakeTransform` (0.0 0.0 0.0)) "AdjustIfPossibleButAlwaysSpawn" "MultiplyWithRoot" null self null))
  (set `self.SpearReference` _returnvalue)
  (set `/Game/Blueprints/Enemies/GaolSpearGuard_Rework/Actions/EA_REW_GaolSpearGuard_SwingStumble.ownerSpearReference` (`self.SpearReference`) (`self.EA_REW_GaolSpearGuard_SwingStumble`)))

(event `self.ReceiveTick`
  (params (DeltaSeconds :type "Float (single-precision)"))
  (`parent.ReceiveTick` DeltaSeconds)
  (`self.UpdateEquipment`))

(event `self.PopulateActionList`
  (`BlueprintMapLibrary.Map_Add` (`self.ActionList`) "IDLE" (`self.EA_REW_GaolSpearGuard_Idle`))
  (`BlueprintMapLibrary.Map_Add` (`self.ActionList`) "CHASE" (`self.EA_REW_GaolSpearGuard_Chase`))
  (`BlueprintMapLibrary.Map_Add` (`self.ActionList`) "SWINGSTUMBLE" (`self.EA_REW_GaolSpearGuard_SwingStumble`)))

(event `self.KillCleanupEvent`
  (`self.K2_DestroyActor` (`self.SpearReference`)))

(fn `UpdateEquipment`
  (bind (_returnvalue_location _returnvalue_rotation) (`KismetMathLibrary.BreakTransform` (`SkinnedMeshComponent.GetBoneTransform` (`self.Mesh`) "Bone_008" "RTS_World")))
  (`self.K2_SetActorLocationAndRotation` (`self.SpearReference`) (+ _returnvalue_location (* (`KismetMathLibrary.GetRightVector` _returnvalue_rotation) -15.0)) _returnvalue_rotation true false)
  (return))

(fn `UserConstructionScript`
  (bind _ea_rew_gaolspearguard_idle (`self.EA_REW_GaolSpearGuard_Idle`))
  (`parent.UserConstructionScript`)
  (bind _output_get (set `self.entryState` _ea_rew_gaolspearguard_idle))
  (set `self.currentState` _output_get)
  (set `EnemyAction.isActiveState` true _ea_rew_gaolspearguard_idle)
  (`self.PopulateActionList`))