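; BP_GaolSpearGuard is a spear-wielding enemy whose behavior is built from named action states, including idle, chase, five attacks and tether return.
; Construction fills the action list, starts in idle and applies wander speed.
; BeginPlay spawns a spear shared with each attack, Tick sweeps it to an offset hand-bone transform instead of attaching it, and kill cleanup destroys it.
; Hitting the tether limit forces a move back to the tether position, then idle.
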(event `self.ReceiveBeginPlay`
  (`parent.ReceiveBeginPlay`)
  (bind _returnvalue (`|SpawnActorFromClass` "/Game/Blueprints/Items/Weapons/NewWeapons/BP_GuardSpear.BP_GuardSpear_C" (`KismetMathLibrary.MakeTransform` (0.0 0.0 0.0)) "AdjustIfPossibleButAlwaysSpawn" "MultiplyWithRoot" null self null))
  (bind _output_get (set `self.SpearReference` _returnvalue))
  (bind _output_get_2 (set `/Game/Blueprints/Enemies/GaolSpearGuard/Actions/EA_GaolSpearGuard_Thrust.OwnerSpearReference` _output_get (`self.EA_GaolSpearGuard_Thrust`)))
  (bind _output_get_3 (set `/Game/Blueprints/Enemies/GaolSpearGuard/Actions/EA_GaolSpearGuard_SpearSpin.OwnerSpearReference` _output_get_2 (`self.EA_GaolSpearGuard_SpearSpin`)))
  (bind _output_get_4 (set `/Game/Blueprints/Enemies/GaolSpearGuard/Actions/EA_GaolSpearGuard_FlyingStrike.OwnerSpearReference` _output_get_3 (`self.EA_GaolSpearGuard_FlyingStrike`)))
  (bind _output_get_5 (set `/Game/Blueprints/Enemies/GaolSpearGuard/Actions/EA_GaolSpearGuard_PoundToSwing.OwnerSpearReference` _output_get_4 (`self.EA_GaolSpearGuard_PoundToSwing`)))
  (set `/Game/Blueprints/Enemies/GaolSpearGuard/Actions/EA_GaolSpearGuard_BackstepStab.OwnerSpearReference` _output_get_5 (`self.EA_GaolSpearGuard_BackstepStab`)))

(event `self.ReceiveTick`
  (params (DeltaSeconds :type "Float (single-precision)"))
  (`parent.ReceiveTick` DeltaSeconds)
  (`self.UpdateEquipment`))

(event `self.PopulateActionList`
  (`BlueprintMapLibrary.Map_Add` (`self.ActionList`) "IDLE" (`self.EA_GaolSpearGuard_Idle`))
  (`BlueprintMapLibrary.Map_Add` (`self.ActionList`) "CHASE" (`self.EA_GaolSpearGuard_Chase`))
  (`BlueprintMapLibrary.Map_Add` (`self.ActionList`) "THRUST" (`self.EA_GaolSpearGuard_Thrust`))
  (`BlueprintMapLibrary.Map_Add` (`self.ActionList`) "SPIN" (`self.EA_GaolSpearGuard_SpearSpin`))
  (`BlueprintMapLibrary.Map_Add` (`self.ActionList`) "FLYINGSTRIKE" (`self.EA_GaolSpearGuard_FlyingStrike`))
  (`BlueprintMapLibrary.Map_Add` (`self.ActionList`) "POUNDSWING" (`self.EA_GaolSpearGuard_PoundToSwing`))
  (`BlueprintMapLibrary.Map_Add` (`self.ActionList`) "BACKSTEPSTAB" (`self.EA_GaolSpearGuard_BackstepStab`))
  (`BlueprintMapLibrary.Map_Add` (`self.ActionList`) "TETHERRETURN" (`self.EA_GaolSpearGuard_TetherReturn`)))

(event `self.KillCleanupEvent`
  (`self.K2_DestroyActor` (`self.SpearReference`)))

(event `self.TetherLimitReached`
  (`|AIMoveTo` self (`self.tetherPosition`) null 100.0
    (:`then`
      (`self.NextState` (`self.EA_GaolSpearGuard_TetherReturn`) true)
      (`KismetSystemLibrary.PrintString` "tethered"))
    (:`OnSuccess`
      (`self.NextState` (`self.EA_GaolSpearGuard_Idle`) true)
      (`KismetSystemLibrary.PrintString` "reach"))
    (:`OnFail`
      (`self.NextState` (`self.EA_GaolSpearGuard_Idle`) true)
      (`KismetSystemLibrary.PrintString` "no valid tether path"))))

(fn `UpdateEquipment`
  (bind (_returnvalue_location _returnvalue_rotation) (`KismetMathLibrary.BreakTransform` (`SkinnedMeshComponent.GetBoneTransform` (`self.Mesh`) "Bone_008" "RTS_World")))
  (`self.K2_SetActorLocationAndRotation` (`self.SpearReference`) (+ _returnvalue_location (* (`KismetMathLibrary.GetRightVector` _returnvalue_rotation) -15.0)) _returnvalue_rotation true false)
  (return))

(fn `UserConstructionScript`
  (`parent.UserConstructionScript`)
  (bind _output_get (set `self.entryState` (`self.EA_GaolSpearGuard_Idle`)))
  (set `self.currentState` _output_get)
  (`self.PopulateActionList`)
  (set `CharacterMovementComponent.MaxWalkSpeed` (`self.wanderSpeed`) (`self.CharacterMovement`)))