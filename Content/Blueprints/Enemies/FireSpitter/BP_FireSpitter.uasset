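; BP_FireSpitter is the Fire Spitter enemy, driven by a set of switchable action states.
; The construction script sets Idle as the entry and current state, then fills a named action list with Idle, Chase, Spark Orb and Flying Beam actions.
; BeginPlay switches into the entry state by reference after the parent's setup.
; Tick only calls the parent, and no transitions between actions are defined in these graphs.
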(event `self.ReceiveBeginPlay`
  (`parent.ReceiveBeginPlay`)
  (`/Game/Blueprints/Enemies/BP_EnemyAction.SwitchToStateByReference` (`self.EA_Firespitter_Idle`) (`self.entryState`)))

(event `self.ReceiveTick`
  (params (DeltaSeconds :type "Float (single-precision)"))
  (`parent.ReceiveTick` DeltaSeconds))

(event `self.PopulateActionList`
  (`BlueprintMapLibrary.Map_Add` (`self.ActionList`) "IDLE" (`self.EA_Firespitter_Idle`))
  (`BlueprintMapLibrary.Map_Add` (`self.ActionList`) "CHASE" (`self.EA_Firespitter_Chase`))
  (`BlueprintMapLibrary.Map_Add` (`self.ActionList`) "SPARKS" (`self.EA_Firespitter_SparkOrb`))
  (`BlueprintMapLibrary.Map_Add` (`self.ActionList`) "FLYINGBEAM" (`self.EA_Firespitter_FlyingBeam`)))

(fn `UserConstructionScript`
  (`parent.UserConstructionScript`)
  (bind _output_get (set `self.entryState` (`self.EA_Firespitter_Idle`)))
  (set `self.currentState` _output_get)
  (`self.PopulateActionList`))