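; Anim notify state that opens a rotation window on an enemy during part of an animation, by its name for turning toward the player.
; On begin it casts the mesh owner to BP_EnemyCharacter, enables CanRotate on its CurrentState and sets that state's MaxRotationSpeed from the notify's RotationSpeed.
; On end it disables CanRotate; the turning itself happens outside this asset.
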(fn `Received_NotifyBegin`
  (params (MeshComp :type "SkeletalMeshComponent Object Reference") (Animation :type "AnimSequenceBase Object Reference") (TotalDuration :type "Float (single-precision)") (EventReference :type "AnimNotifyEventReference Structure (by ref)"))
  (returns (ReturnValue :type Boolean))
  (bind _asbp_enemy_character (cast `/Game/Blueprints/Enemies/BP_EnemyCharacter` (`ActorComponent.GetOwner` MeshComp)))
  (bind _currentstate (`EnemyCharacter.currentState` _asbp_enemy_character))
  (set `EnemyAction.canRotate` true _currentstate)
  (set `EnemyAction.maxRotationSpeed` (`self.rotationSpeed`) _currentstate)
  (return false))

(fn `Received_NotifyEnd`
  (params (MeshComp :type "SkeletalMeshComponent Object Reference") (Animation :type "AnimSequenceBase Object Reference") (EventReference :type "AnimNotifyEventReference Structure (by ref)"))
  (returns (ReturnValue :type Boolean))
  (bind _asbp_enemy_character (cast `/Game/Blueprints/Enemies/BP_EnemyCharacter` (`ActorComponent.GetOwner` MeshComp)))
  (set `EnemyAction.canRotate` false (`EnemyCharacter.currentState` _asbp_enemy_character))
  (return false))