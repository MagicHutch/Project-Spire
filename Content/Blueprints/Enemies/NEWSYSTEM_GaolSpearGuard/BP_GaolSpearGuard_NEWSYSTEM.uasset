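; Gaol spear guard enemy that fights with a spear and shield, built on a parent state-driven entity class.
; On BeginPlay it registers swing, thrust, wander, seek, face-player and shield-bash states, enters at wander, and spawns both weapons, with the spear ignoring its own class.
; Each tick it sweeps the separate spear and shield actors to offset hand-placed bone transforms instead of attaching them.
; KillEntity destroys both equipment actors along with the guard.
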(event `self.ReceiveBeginPlay`
  (bind _returnvalue (`self.GetTransform`))
  ;[1 1 1] Begin
  (`self.InitializeStateList`)
  (set `self.entryState` (`BlueprintMapLibrary.Map_Find` (`self.stateList`) 2))
  (bind _returnvalue_2 (`|SpawnActorFromClass` "/Game/Blueprints/Items/Weapons/NewWeapons/BP_GuardSpear.BP_GuardSpear_C" _returnvalue "Undefined" "MultiplyWithRoot" null null))
  (bind _output_get (set `self.SpearReference` _returnvalue_2))
  (`/Game/Blueprints/Items/Weapons/NewWeapons/BP_UsableWeapon.Configure Ignore Classes` _output_get (`|MakeArray` "BP_GaolSpearGuard_NEWSYSTEM_C" :!type "Actor Class Reference"))
  (bind _returnvalue_3 (`|SpawnActorFromClass` "/Game/Blueprints/Items/Weapons/OldWeapons/BP_BasicShield.BP_BasicShield_C" _returnvalue "Undefined" "MultiplyWithRoot" null null))
  (set `self.ShieldReference` _returnvalue_3)
  (`parent.ReceiveBeginPlay`))

(event `self.ReceiveTick`
  (params (DeltaSeconds :type "Float (single-precision)"))
  (`parent.ReceiveTick` DeltaSeconds)
  (`self.UpdateEquipment`))

(event `UpdateEquipment`
  (bind _mesh (`self.Mesh`))
  (bind (_returnvalue_location _returnvalue_rotation) (`KismetMathLibrary.BreakTransform` (`SkinnedMeshComponent.GetBoneTransform` _mesh "Bone_005" "RTS_World")))
  (bind (_returnvalue_location_2 _returnvalue_rotation_2) (`KismetMathLibrary.BreakTransform` (`SkinnedMeshComponent.GetBoneTransform` _mesh "Bone_008" "RTS_World")))
  ;[1 1 1] Update Equipment
  ;;[1 1 1] Spear
  (`self.K2_SetActorLocationAndRotation` (`self.SpearReference`) (+ _returnvalue_location_2 (* (`KismetMathLibrary.GetRightVector` _returnvalue_rotation_2) -15.0)) _returnvalue_rotation_2 true false)
  ;;[1 1 1] Shield
  (`self.K2_SetActorLocationAndRotation` (`self.ShieldReference`) (+ _returnvalue_location (+ (* (`KismetMathLibrary.GetRightVector` _returnvalue_rotation) -15.0) (* (`KismetMathLibrary.GetForwardVector` _returnvalue_rotation) -15.0))) _returnvalue_rotation true false))

(event `self.KillEntity`
  ;[1 1 1] Destroy Function
  (`self.K2_DestroyActor` (`self.SpearReference`))
  (`self.K2_DestroyActor` (`self.ShieldReference`))
  (`self.K2_DestroyActor`))

(fn `InitializeStateList`
  (bind _statelist (`self.stateList`))
  (`BlueprintMapLibrary.Map_Add` _statelist 0 (`self.EA_NEWGaolSpearGuard_SWING`))
  (`BlueprintMapLibrary.Map_Add` _statelist 1 (`self.EA_NEWGaolSpearGuard_Thrust`))
  (`BlueprintMapLibrary.Map_Add` _statelist 2 (`self.EA_NEWGaolSpearGuard_Wander`))
  (`BlueprintMapLibrary.Map_Add` _statelist 3 (`self.EA_NEWGaolSpearGuard_Seek`))
  (`BlueprintMapLibrary.Map_Add` _statelist 4 (`self.EA_NEWGaolSpearGuard_FacePlayer`))
  (`BlueprintMapLibrary.Map_Add` _statelist 5 (`self.EA_NEWGaolSpearGuard_ShieldBash`)))

(fn `UserConstructionScript`
  (`parent.UserConstructionScript`))