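; Base enemy action that caches its owning enemy character and provides shared helpers around an empty UseAction event.
; Player checks cover view cone with range limit, distance and height difference.
; State switches pass a state, given directly or looked up by name in the owner's ActionList, to NextState.
; Movement helpers apply clamped yaw toward the player or synchronously find a path and steer toward its first useful point, drawing a debug arrow.
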(event `self.ReceiveBeginPlay`
  (bind _asenemy_character (cast `EnemyCharacter` (`self.GetOwner`)))
  (bind _output_get (set `self.Owner` _asenemy_character))
  (set `self.OwnerSkeletalMesh` (`Actor.GetComponentByClass` _output_get "/Script/Engine.SkeletalMeshComponent"))
  (bind _asbp_enemy_character (cast `/Game/Blueprints/Enemies/BP_EnemyCharacter` _output_get))
  (set `self.OwnerBlueprint` _asbp_enemy_character))

(event `self.UseAction`)

(fn `NavigateToActor`
  (params (ActorToNavigateTo :type "Actor Object Reference") (InputPath :type "NavigationPath Object Reference"))
  (returns (OutputPath :type "NavigationPath Object Reference"))
  (bind _owner (`self.Owner`))
  (bind _owner_2 (`self.Owner`))
  (bind _returnvalue (`NavigationSystemV1.FindPathToLocationSynchronously` (`Actor.K2_GetActorLocation` (`self.Owner`)) (`Actor.K2_GetActorLocation` ActorToNavigateTo) null null))
  (bind _pathpoints (`NavigationPath.PathPoints` _returnvalue))
  (for _array_element _pathpoints
    (`KismetSystemLibrary.DrawDebugArrow` _array_element (+ _array_element (0.0 0.0 100.0)) 5.0 (struct :`R` 0.916555 :`B` 1.0 :`A` 1.0) 0.0 2.0)
    (if (< (`KismetMathLibrary.VSize` (- (`|GetArrayItem` _pathpoints) (`Actor.K2_GetActorLocation` _owner))) (+ (`CapsuleComponent.GetScaledCapsuleHalfHeight` (`Character.CapsuleComponent` _owner)) 10.0))
      (`KismetArrayLibrary.Array_Remove` _pathpoints))
    (`Pawn.AddMovementInput` _owner_2 (`KismetMathLibrary.Normal` (- (`|GetArrayItem` (`NavigationPath.PathPoints` _returnvalue)) (`Actor.K2_GetActorLocation` _owner_2))) 1.0 false)
    (return null)))

(fn `PlayerInFieldOfView`
  (returns (inFOV :type Boolean))
  (bind _owner (`self.Owner`))
  (bind _player (`EnemyCharacter.player` _owner))
  (bind _returnvalue (`EnemyCharacter.AngleBetweenVectors` _owner (`KismetMathLibrary.GetForwardVector` (`Actor.K2_GetActorRotation` _owner)) (- (`Actor.K2_GetActorLocation` _player) (`Actor.K2_GetActorLocation` _owner))))
  (if (and (<= _returnvalue (`EnemyCharacter.fieldOfViewAngle` _owner)) (< (`Actor.GetDistanceTo` _owner _player) 1000.0))
    (return true)
    (else
      (return false))))

(fn `PlayerSelfElevationDifference`
  (returns (ElevationDifference :type "Float (double-precision)"))
  (bind _owner (`self.Owner`))
  (bind (_returnvalue_x _returnvalue_y _returnvalue_z) (`KismetMathLibrary.BreakVector` (`Actor.K2_GetActorLocation` _owner)))
  (bind (_returnvalue_x_2 _returnvalue_y_2 _returnvalue_z_2) (`KismetMathLibrary.BreakVector` (`Actor.K2_GetActorLocation` (`EnemyCharacter.player` _owner))))
  (return (`KismetMathLibrary.VSize` (- (`KismetMathLibrary.MakeVector` 0.0 0.0 _returnvalue_z) (`KismetMathLibrary.MakeVector` 0.0 0.0 _returnvalue_z_2)))))

(fn `PlayerWithinDistance`
  (params (Distance :type "Float (double-precision)"))
  (returns (WithinRadius :type Boolean))
  (bind _owner (`self.Owner`))
  (if (<= (`Actor.GetDistanceTo` _owner (`EnemyCharacter.player` _owner)) Distance)
    (return true)
    (else
      (return false))))

(fn `RotateTowardsPlayer`
  (params (MaxRotationPerFrame :type "Float (double-precision)"))
  (bind _owner (`self.Owner`))
  (bind _returnvalue (`EnemyCharacter.AngleToPlayer` _owner))
  (`Actor.K2_AddActorWorldRotation` _owner (`KismetMathLibrary.MakeRotator` 0.0 0.0 (* (`KismetMathLibrary.FClamp` _returnvalue (* MaxRotationPerFrame -1.0) MaxRotationPerFrame) -1.0)) false false))

(fn `SwitchToState`
  (params (StateName :type String))
  (returns (Success :type Boolean))
  (bind _returnvalue (`EnemyCharacter.NextState` (`self.Owner`) (`BlueprintMapLibrary.Map_Find` (`/Game/Blueprints/Enemies/BP_EnemyCharacter.ActionList` (`self.OwnerBlueprint`)) StateName)))
  (return _returnvalue))

(fn `SwitchToStateByReference`
  (params (`New State` :type "EnemyAction Object Reference"))
  (returns (Success :type Boolean))
  (bind _returnvalue (`EnemyCharacter.NextState` (`self.Owner`) `New State`))
  (return _returnvalue))