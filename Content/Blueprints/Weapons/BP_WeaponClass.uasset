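; BP_WeaponClass is a melee weapon actor that deals damage through a traced hitbox while an attack is active.
; Each tick during an attack, it sphere-traces for Pawns along its up vector.
; Hit actors take raw damage and join an ignore list to prevent repeat hits, while "Shield"-tagged actors end the attack as blocked.
; Deactivation resets that list to all instances of the configured ignored classes.
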(event `self.ReceiveBeginPlay`
  (`self.Set Ignore Actors` (`self.ActorClassesToIgnore`)))

(event `self.ReceiveTick`
  (params (DeltaSeconds :type "Float (single-precision)"))
  (`self.Use Attack` (`self.ActorsToIgnore`)))

(event `Activate Attack`
  ;[1 1 1] Activate
  (set `self.Is Attacking` true))

(event `Deactivate Attack`
  ;[1 1 1] Deactivate
  (set `self.Is Attacking` false)
  (`KismetArrayLibrary.Array_Clear` (`self.ActorsToIgnore`))
  (`self.Set Ignore Actors` (`self.ActorClassesToIgnore`)))

(event `Set Ignore Actors`
  (params (Actors :type "Array of Actor Class Reference"))
  ;[1 1 1] Set Ignore Actors
  (for _array_element Actors
    (bind _outactors (`GameplayStatics.GetAllActorsOfClass` _array_element))
    (for _array_element_2 _outactors
      (`KismetArrayLibrary.Array_Add` (`self.ActorsToIgnore`) _array_element_2))))

(event `Use Attack`
  (params (ActorsToIgnore :type "Array of Actor Object Reference"))
  (bind _returnvalue_location (`KismetMathLibrary.BreakTransform` (`self.GetTransform`)))
  ;[1 1 1] UseAttack
  (if (`self.Is Attacking`)
    (bind (_outhit _returnvalue) (`KismetSystemLibrary.SphereTraceSingleForObjects` _returnvalue_location (+ _returnvalue_location (* (`self.GetActorUpVector`) (`self.HitboxLength`))) (`self.HitboxRadius`) (`|MakeArray` "ObjectTypeQuery3" :!type "EObjectTypeQuery Enum") false ActorsToIgnore "ForOneFrame"))
    (if _returnvalue
      (bind (_bblockinghit _binitialoverlap _time _distance _location _impactpoint _normal _impactnormal _physmat _hitactor) (`GameplayStatics.BreakHitResult` _outhit))
      (if (`self.ActorHasTag` _hitactor "Shield")
        (`self.Deactivate Attack`)
        (`KismetSystemLibrary.PrintString` "Attack Blocked")
        (else
          (`GameplayStatics.ApplyDamage` _hitactor (`self.RawDamage`))
          (`KismetArrayLibrary.Array_Add` (`self.ActorsToIgnore`) _hitactor))))))

(fn `UserConstructionScript`)