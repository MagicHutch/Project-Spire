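; BP_BasicSword is a melee sword actor that kills pawns it hits during an attack.
; While IsAttacking is set, Tick runs a short debug-drawn sphere trace along the sword's up vector, looking for Pawn objects and ignoring the player pawn.
; A hit destroys that actor outright, with no damage step, then calls InitLockOn on BP_Player.
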(event `self.ReceiveTick`
  (params (DeltaSeconds :type "Float (single-precision)"))
  (bind _returnvalue_location (`KismetMathLibrary.BreakTransform` (`self.GetTransform`)))
  (if (`self.Is Attacking`)
    (bind (_outhit _returnvalue) (`KismetSystemLibrary.SphereTraceSingleForObjects` _returnvalue_location (+ _returnvalue_location (* (`self.GetActorUpVector`) 50.0)) 20.0 (`|MakeArray` "ObjectTypeQuery3" :!type "EObjectTypeQuery Enum") false (`|MakeArray` (`GameplayStatics.GetPlayerPawn` 0) :!type "Actor Object Reference") "ForDuration"))
    (if _returnvalue
      (`self.K2_DestroyActor` (`.HitActor` (`GameplayStatics.BreakHitResult` _outhit)))
      (bind _returnvalue_2 (`GameplayStatics.GetActorOfClass` "/Game/Blueprints/BP_Player.BP_Player_C"))
      (`/Game/Blueprints/BP_Player.Init LockOn` _returnvalue_2))))

(fn `UserConstructionScript`)