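; BP_SpearLightningPulse is a short-lived area-of-effect lightning pulse that damages actors it touches, sparing the player.
; On BeginPlay it adds the first player's pawn to ActorsToIgnore, then destroys itself after TimeToPersist.
; Any actor that begins overlapping the LightningBlast component and is not on that list takes DamageToDeal damage.
; Hit actors are not added to the list, so re-entering the blast damages them again.
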(event `self.ReceiveBeginPlay`
  (`KismetArrayLibrary.Array_Add` (`self.ActorsToIgnore`) (`GameplayStatics.GetPlayerPawn` 0))
  (`KismetSystemLibrary.Delay` (`self.TimeToPersist`))
  (`self.K2_DestroyActor`))

(event `self.LightningBlast.OnComponentBeginOverlap`
  (params (OverlappedComponent :type "PrimitiveComponent Object Reference") (OtherActor :type "Actor Object Reference") (OtherComp :type "PrimitiveComponent Object Reference") (OtherBodyIndex :type Integer) (bFromSweep :type Boolean) (SweepResult :type "HitResult Structure (by ref)"))
  (if (not (`KismetArrayLibrary.Array_Contains` (`self.ActorsToIgnore`) OtherActor))
    (`GameplayStatics.ApplyDamage` OtherActor (`self.DamageToDeal`))))

(fn `UserConstructionScript`)