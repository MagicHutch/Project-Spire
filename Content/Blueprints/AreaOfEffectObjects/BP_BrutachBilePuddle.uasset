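; Brutach bile puddle area-of-effect actor that builds up Despair on characters standing in it.
; On spawn it prints a debug string and adjusts to the closest floor.
; Puddle overlaps run shared begin/end processing and track actors with CharacterStats, excluding the source actor, in AffectedActors.
; Each tick raises their Despair meter by a per-second rate scaled by delta time, skipping anyone already afflicted with Despair.
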(event `self.ReceiveBeginPlay`
  (`parent.ReceiveBeginPlay`)
  (`KismetSystemLibrary.PrintString` "puddle spawned")
  (`self.AdjustToClosestFloor` -1))

(event `self.ReceiveTick`
  (params (DeltaSeconds :type "Float (single-precision)"))
  (`parent.ReceiveTick` DeltaSeconds)
  (`self.DespairBuildupTick` DeltaSeconds))

(event `self.Puddle.OnComponentBeginOverlap`
  (params (OverlappedComponent :type "PrimitiveComponent Object Reference") (OtherActor :type "Actor Object Reference") (OtherComp :type "PrimitiveComponent Object Reference") (OtherBodyIndex :type Integer) (bFromSweep :type Boolean) (SweepResult :type "HitResult Structure (by ref)"))
  (bind _affectedactors (`self.AffectedActors`))
  (`self.ProcessBeginOverlap` OtherActor OtherComp)
  (if (and (`KismetSystemLibrary.IsValid` (`self.GetComponentByClass` OtherActor "/Script/MyProject.CharacterStats")) (!= OtherActor (`self.sourceActor`)))
    (if (not (`KismetArrayLibrary.Array_Contains` _affectedactors OtherActor))
      (`KismetArrayLibrary.Array_Add` _affectedactors OtherActor))))

(event `self.Puddle.OnComponentEndOverlap`
  (params (OverlappedComponent :type "PrimitiveComponent Object Reference") (OtherActor :type "Actor Object Reference") (OtherComp :type "PrimitiveComponent Object Reference") (OtherBodyIndex :type Integer))
  (`self.ProcessEndOverlap` OtherActor)
  (`KismetArrayLibrary.Array_RemoveItem` (`self.AffectedActors`) OtherActor))

(fn `DespairBuildupTick`
  (params (inDeltaTime :type "Float (double-precision)"))
  (for _array_element (`self.AffectedActors`)
    (bind _returnvalue (`self.GetComponentByClass` _array_element "/Script/MyProject.CharacterStats"))
    (if (`KismetSystemLibrary.IsValid` _returnvalue)
      (if (not (`BlueprintMapLibrary.Map_Find` (`CharacterStats.appliedStatusConditions` _returnvalue) "DESPAIR"))
        (`CharacterStats.IncreaseDespairMeter` _returnvalue (* (`local.inDeltaTime`) (`self.DespairBuildupPerSecond`)))))))

(fn `UserConstructionScript`
  (`parent.UserConstructionScript`))