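; BP_WeaponAreaOfEffect is a weapon damage area that hurts damageable actors it overlaps, initially ignoring its source actor.
; Overlap handlers apply damage once per entry via an ignore list cleared on exit, and players are only hit through their current damage hitbox.
; It destroys itself after its duration, with Tick handling zero duration as a single active frame.
; A helper snaps it vertically onto nearby static geometry with a line trace.
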(event `self.ReceiveBeginPlay`
  (`KismetSystemLibrary.Delay` (`self.duration`))
  (`self.K2_DestroyActor`))

(event `self.ReceiveTick`
  (params (DeltaSeconds :type "Float (single-precision)"))
  (if (== (`self.duration`) 0.0)
    (if (`self.activeForFrame`)
      (`self.K2_DestroyActor`)
      (else
        (set `self.activeForFrame` true)))))

(fn `AdjustToClosestFloor`
  (params (castDirection :type Integer))
  (bind _returnvalue (`self.K2_GetActorLocation`))
  (bind (_returnvalue_x _returnvalue_y) (`KismetMathLibrary.BreakVector` (`self.K2_GetActorLocation`)))
  (bind (_outhit _returnvalue_2) (`KismetSystemLibrary.LineTraceSingleForObjects` _returnvalue (+ _returnvalue (`KismetMathLibrary.MakeVector` 0.0 0.0 (* 600.0 (`local.castDirection`)))) (`|MakeArray` "ObjectTypeQuery1" :!type "EObjectTypeQuery Enum")))
  (if _returnvalue_2
    (`self.K2_SetActorLocation` (`KismetMathLibrary.MakeVector` _returnvalue_x _returnvalue_y (.z (`.Location` (`GameplayStatics.BreakHitResult` _outhit)))) false true)))

(fn `ProcessBeginOverlap`
  (params (InOtherActor :type "Actor Object Reference") (InOtherComp :type "PrimitiveComponent Object Reference"))
  (if (not (`KismetArrayLibrary.Array_Contains` (`self.actorsToIgnore`) (`local.InOtherActor`)))
    (if (`Actor.bCanBeDamaged` (`local.InOtherActor`))
      (bind _asbp_player_v3 (cast `/Game/Blueprints/Player/BP_PlayerV3` (`local.InOtherActor`))
        (:`then`
          (if (== (`/Game/Blueprints/Player/BP_PlayerV3.currentDamageHitbox` _asbp_player_v3) (`local.InOtherComp`))
            (`GameplayStatics.ApplyDamage` (`local.InOtherActor`) (`self.damageToDeal`) :!label _label)
            (`KismetArrayLibrary.Array_Add` (`self.actorsToIgnore`) (`local.InOtherActor`))))
        (:`CastFailed`
          (goto _label))))))

(fn `ProcessEndOverlap`
  (params (InOtherActor :type "Actor Object Reference"))
  (if (`KismetArrayLibrary.Array_Contains` (`self.actorsToIgnore`) (`local.InOtherActor`))
    (`KismetArrayLibrary.Array_RemoveItem` (`self.actorsToIgnore`) (`local.InOtherActor`))))

(fn `UserConstructionScript`
  (`KismetArrayLibrary.Array_Add` (`self.actorsToIgnore`) (`self.sourceActor`)))