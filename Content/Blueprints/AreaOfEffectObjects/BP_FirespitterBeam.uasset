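; Firespitter beam area-of-effect actor that sizes a fire beam to the world geometry in its path.
; On BeginPlay it line-traces static world objects along BeamDirection from StartPosition and stretches the FireBeam component's Z scale to the hit distance, using a fixed scale on a miss.
; FireBeam begin and end overlaps feed the ProcessBeginOverlap and ProcessEndOverlap handlers.
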(event `self.ReceiveBeginPlay`
  (bind _startposition (`self.startPosition`))
  (`parent.ReceiveBeginPlay`)
  (bind (_outhit _returnvalue) (`KismetSystemLibrary.LineTraceSingleForObjects` _startposition (+ _startposition (* (`self.beamDirection`) 1500.0)) (`|MakeArray` "ObjectTypeQuery1" :!type "EObjectTypeQuery Enum")))
  (if _returnvalue
    (`SceneComponent.SetRelativeScale3D` (`self.FireBeam`) (`KismetMathLibrary.MakeVector` 1.0 1.0 (/ (`KismetMathLibrary.Vector_Distance` (`self.startPosition`) (`.Location` (`GameplayStatics.BreakHitResult` _outhit))) 100.0)))
    (else
      (`SceneComponent.SetRelativeScale3D` (`self.FireBeam`) (1.0 1.0 1.5)))))

(event `self.ReceiveTick`
  (params (DeltaSeconds :type "Float (single-precision)"))
  (`parent.ReceiveTick` DeltaSeconds))

(event `self.FireBeam.OnComponentBeginOverlap`
  (params (OverlappedComponent :type "PrimitiveComponent Object Reference") (OtherActor :type "Actor Object Reference") (OtherComp :type "PrimitiveComponent Object Reference") (OtherBodyIndex :type Integer) (bFromSweep :type Boolean) (SweepResult :type "HitResult Structure (by ref)"))
  (`self.ProcessBeginOverlap` OtherActor OtherComp))

(event `self.FireBeam.OnComponentEndOverlap`
  (params (OverlappedComponent :type "PrimitiveComponent Object Reference") (OtherActor :type "Actor Object Reference") (OtherComp :type "PrimitiveComponent Object Reference") (OtherBodyIndex :type Integer))
  (`self.ProcessEndOverlap` OtherActor))

(fn `UserConstructionScript`
  (`parent.UserConstructionScript`))