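; BP_ItemPickup is an item pickup that the player can interact with while overlapping it.
; It caches the player pawn as BP_PlayerV2 on BeginPlay.
; Overlap begin sets the pickup as the player's InteractObject, and overlap end clears that reference.
; The UsePickup event only destroys the actor, and nothing in this file calls it.
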(event `self.ReceiveBeginPlay`
  (bind _asbp_player_v2 (cast `/Game/Blueprints/Player/BP_PlayerV2` (`GameplayStatics.GetPlayerPawn` 0)))
  (set `self.Player` _asbp_player_v2))

(event `self.ReceiveActorBeginOverlap`
  (params (OtherActor :type "Actor Object Reference"))
  (bind _player (`self.Player`))
  (if (== OtherActor _player)
    (set `/Game/Blueprints/Player/BP_PlayerV2.InteractObject` self _player)))

(event `self.ReceiveActorEndOverlap`
  (params (OtherActor :type "Actor Object Reference"))
  (bind _player (`self.Player`))
  (if (== OtherActor _player)
    (set `/Game/Blueprints/Player/BP_PlayerV2.InteractObject` null _player)))

(event `UsePickup`
  (`self.K2_DestroyActor`))

(fn `UserConstructionScript`)