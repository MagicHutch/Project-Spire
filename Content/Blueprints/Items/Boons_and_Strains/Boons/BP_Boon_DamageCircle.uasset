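; Damage circle boon that, when used, places a temporary zone beneath the player; no damage is applied in this Blueprint.
; UseSkill teleports the actor below the player's capsule centre and activates it for CircleLifespan, then deactivates it and clears ContainedActors.
; Trigger overlaps add actors to that list only while active and remove them on exit.
; The ring is a debug-drawn circle sized from the Trigger's X scale.
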(event `self.ReceiveTick`
  (params (DeltaSeconds :type "Float (single-precision)")))

(event `self.UseSkill`
  (`self.FindSpawnPosition`)
  (set `self.isActive` true)
  (`self.DrawVisualCircle` (`self.circleLifespan`))
  (`KismetSystemLibrary.Delay` (`self.circleLifespan`))
  (set `self.isActive` false)
  (`KismetArrayLibrary.Array_Clear` (`self.containedActors`)))

(event `self.Trigger.OnComponentBeginOverlap`
  (params (OverlappedComponent :type "PrimitiveComponent Object Reference") (OtherActor :type "Actor Object Reference") (OtherComp :type "PrimitiveComponent Object Reference") (OtherBodyIndex :type Integer) (bFromSweep :type Boolean) (SweepResult :type "HitResult Structure (by ref)"))
  (bind _containedactors (`self.containedActors`))
  (if (`self.isActive`)
    (if (not (`KismetArrayLibrary.Array_Contains` _containedactors OtherActor))
      (`KismetArrayLibrary.Array_Add` _containedactors OtherActor))))

(event `self.Trigger.OnComponentEndOverlap`
  (params (OverlappedComponent :type "PrimitiveComponent Object Reference") (OtherActor :type "Actor Object Reference") (OtherComp :type "PrimitiveComponent Object Reference") (OtherBodyIndex :type Integer))
  (bind _containedactors (`self.containedActors`))
  (if (`KismetArrayLibrary.Array_Contains` _containedactors OtherActor)
    (`KismetArrayLibrary.Array_RemoveItem` _containedactors OtherActor)))

(fn `DrawVisualCircle`
  (params (lifeSpan :type "Float (double-precision)"))
  (bind _returnvalue (`SceneComponent.K2_GetComponentToWorld` (`self.Trigger`)))
  (`KismetSystemLibrary.DrawDebugCircle` (.location _returnvalue) (* (/ (.x (.scale _returnvalue)) 2.0) 100.0) 12 (struct :`R` 0.505208 :`B` 0.025913 :`A` 1.0) lifeSpan 2.0 (1.0 0.0 0.0) (0.0 1.0 0.0)))

(fn `FindSpawnPosition`
  (bind _asbp_player_v3 (cast `/Game/Blueprints/Player/BP_PlayerV3` (`GameplayStatics.GetPlayerPawn` 0)))
  (bind (_returnvalue_x _returnvalue_y _returnvalue_z) (`KismetMathLibrary.BreakVector` (`self.K2_GetActorLocation` _asbp_player_v3)))
  (`self.K2_SetActorLocation` (`KismetMathLibrary.MakeVector` _returnvalue_x _returnvalue_y (- _returnvalue_z (`CapsuleComponent.GetScaledCapsuleHalfHeight_WithoutHemisphere` (`Character.CapsuleComponent` _asbp_player_v3)))) false true))

(fn `UserConstructionScript`)