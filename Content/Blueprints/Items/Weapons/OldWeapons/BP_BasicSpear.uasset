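; BP_BasicSpear is a throwable spear weapon that destroys itself on contact with actors not tagged Shield.
; ThrowSpear stores the throw direction and clears IsHeld, ignoring its StartRotation input.
; Tick then moves the spear by a swept, per-frame offset that is not scaled by delta time.
; GravityFactor accumulates during flight, but the node applying it to the direction is disconnected, so flight stays straight.
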(event `self.ReceiveActorBeginOverlap`
  (params (OtherActor :type "Actor Object Reference"))
  (`parent.ReceiveActorBeginOverlap` OtherActor)
  (if (not (`self.ActorHasTag` OtherActor "Shield"))
    (`self.K2_DestroyActor`)))

(event `self.ReceiveTick`
  (params (DeltaSeconds :type "Float (single-precision)"))
  (`parent.ReceiveTick` DeltaSeconds)
  (if (not (`self.IsHeld`))
    (bind _output_get (set `self.GravityFactor` (- (`self.GravityFactor`) (* DeltaSeconds -9.8))))
    (bind _sweephitresult (`self.K2_AddActorWorldOffset` (`self.FlightDirection`) true))
    (bind (_bblockinghit _binitialoverlap _time _distance _location _impactpoint _normal _impactnormal _physmat _hitactor) (`GameplayStatics.BreakHitResult` _sweephitresult))
    (if _bblockinghit
      (if (not (`self.ActorHasTag` _hitactor "Shield"))
        (`self.K2_DestroyActor`)))))

(event `Throw Spear`
  (params (StartRotation :type "Rotator Structure") (ThrowDirection :type "Vector Structure"))
  (set `self.FlightDirection` ThrowDirection)
  (set `self.IsHeld` false))

(fn `UserConstructionScript`
  (`parent.UserConstructionScript`))