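; Guard spear weapon Blueprint whose right-hand stab animations change with its weapon level.
; When the level is altered, it prints the new level and toggles a light handle upgrade that is active from level three upward.
; The upgrade overwrites the first two right stab sequence entries with the RMED stab montage, while lower levels restore the RHEV version.
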(event `self.ReceiveTick`
  (params (DeltaSeconds :type "Float (single-precision)"))
  (`parent.ReceiveTick` DeltaSeconds))

(event `self.AlterLevel`
  (bind _weaponlevel (`self.weaponLevel`))
  (`|ExecutionSequence`
    (:`then_0`
      (`KismetSystemLibrary.PrintString` (`KismetTextLibrary.Conv_TextToString` (`|FormatText` "alter weapon level, new: {0}" _weaponlevel)))
      (if (>= _weaponlevel 3)
        (`self.ToggleLightHandleUpgrade` true)
        (else
          (`self.ToggleLightHandleUpgrade` false))))))

(fn `ToggleLightHandleUpgrade`
  (params (hasLightHandle :type Boolean))
  (if hasLightHandle
    (`KismetArrayLibrary.Array_Set` (`self.rightStabSequence`) 0 "/Game/Characters/HumanMaleTest/NewAttackAnims/Montages/AM_PlayerV3_RMED_Stab01.AM_PlayerV3_RMED_Stab01")
    (`KismetArrayLibrary.Array_Set` (`self.rightStabSequence`) 1 "/Game/Characters/HumanMaleTest/NewAttackAnims/Montages/AM_PlayerV3_RMED_Stab01.AM_PlayerV3_RMED_Stab01")
    (else
      (`KismetArrayLibrary.Array_Set` (`self.rightStabSequence`) 0 "/Game/Characters/HumanMaleTest/NewAttackAnims/Montages/AM_PlayerV3_RHEV_Stab01.AM_PlayerV3_RHEV_Stab01")
      (`KismetArrayLibrary.Array_Set` (`self.rightStabSequence`) 1 "/Game/Characters/HumanMaleTest/NewAttackAnims/Montages/AM_PlayerV3_RHEV_Stab01.AM_PlayerV3_RHEV_Stab01"))))

(fn `UserConstructionScript`
  (`parent.UserConstructionScript`))