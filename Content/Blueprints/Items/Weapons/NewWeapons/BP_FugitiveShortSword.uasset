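; BP_FugitiveShortSword is a short sword weapon that deals double damage while its owner has the Despair status condition.
; Its DealDamageandUpdateList event looks up Despair in the owner's CharacterStats component and falls back to base damage if the component or condition is absent.
; Each damaged actor is added to ActorsToIgnore.
; The BeginPlay, overlap and Tick events are disabled stubs.
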(event `self.Deal Damage And Update List`
  (params (ActorToDamage :type "Actor Object Reference"))
  (bind _returnvalue (`self.GetComponentByClass` (`self.weaponOwner`) "/Script/MyProject.CharacterStats"))
  (if (`KismetSystemLibrary.IsValid` _returnvalue)
    (if (`BlueprintMapLibrary.Map_Find` (`CharacterStats.appliedStatusConditions` _returnvalue) "DESPAIR")
      (`GameplayStatics.ApplyDamage` ActorToDamage (* (`self.baseDamage`) 2.0) null self)
      (`KismetArrayLibrary.Array_Add` (`self.ActorsToIgnore`) ActorToDamage)
      (else
        (`GameplayStatics.ApplyDamage` ActorToDamage (`self.baseDamage`) null self)
        (`KismetArrayLibrary.Array_Add` (`self.ActorsToIgnore`) ActorToDamage)))
    (else
      (`GameplayStatics.ApplyDamage` ActorToDamage (`self.baseDamage`) null self)
      (`KismetArrayLibrary.Array_Add` (`self.ActorsToIgnore`) ActorToDamage))))

(fn `UserConstructionScript`
  (`parent.UserConstructionScript`))