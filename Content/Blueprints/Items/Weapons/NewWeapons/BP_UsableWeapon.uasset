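; Usable melee weapon that damages pawns through a hitbox active only during attacks.
; Activation sets damage from animation, attack type and weapon level, then gathers existing overlaps.
; New overlaps, filtered to a player's current damage hitbox, join a queue that Tick damages, ignoring each victim until the attack ends.
; The owner and configurable classes are ignored; a separate UseAttack event offers sphere-trace hit detection.
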(event `self.ReceiveBeginPlay`
  (`self.Set Ignore Actors` (`self.ActorClassesToIgnore`))
  (`ActorComponent.Deactivate` (`self.WeaponHitbox`))
  (`SceneComponent.SetVisibility` (`self.WeaponHitbox`) (`self.ShowWeaponHitboxes`) false))

(event `self.ReceiveTick`
  (params (DeltaSeconds :type "Float (single-precision)"))
  (if (`self.IsAttacking`)
    (`self.TickProcessHitActors`)))

(event `self.ActivateAttack`
  (params (isHeavy :type Boolean) (isJump :type Boolean) (isDodge :type Boolean) (isOffhand :type Boolean) (inAnimToCheck :type "AnimMontage Object Reference"))
  ;[1 1 1] Activate
  (`self.SetCurrentDamage` isHeavy isJump isDodge isOffhand inAnimToCheck)
  (set `self.IsAttacking` true)
  (`ActorComponent.Activate` (`self.WeaponHitbox`) true)
  (`self.CheckExistingOverlaps`))

(event `self.DeactivateAttack`
  ;[1 1 1] Deactivate
  (set `self.IsAttacking` false)
  (`KismetArrayLibrary.Array_Clear` (`self.ActorsToIgnore`))
  (`self.Set Ignore Actors` (`self.ActorClassesToIgnore`))
  (`ActorComponent.Deactivate` (`self.WeaponHitbox`)))

(event `Set Ignore Actors`
  (params (Actors :type "Array of Actor Class Reference"))
  ;[1 1 1] Set Ignore Actors
  (`KismetArrayLibrary.Array_Clear` (`self.ActorsToIgnore`))
  (for _array_element Actors
    (bind _outactors (`GameplayStatics.GetAllActorsOfClass` _array_element))
    (for _array_element_2 _outactors
      (`KismetArrayLibrary.Array_Add` (`self.ActorsToIgnore`) _array_element_2)))
  (`KismetArrayLibrary.Array_Add` (`self.ActorsToIgnore`) (`self.weaponOwner`)))

(event `Use Attack`
  (params (ActorsToIgnore :type "Array of Actor Object Reference"))
  (bind _returnvalue_location (`KismetMathLibrary.BreakTransform` (`self.GetTransform`)))
  (bind (_hitboxoffset_x _hitboxoffset_y _hitboxoffset_z) (`KismetMathLibrary.BreakVector` (`self.hitboxOffset`)))
  (bind _returnvalue (+ (+ (+ _returnvalue_location (* (`self.GetActorForwardVector`) _hitboxoffset_x)) (* (`self.GetActorRightVector`) _hitboxoffset_y)) (* (`self.GetActorUpVector`) _hitboxoffset_z)))
  ;[1 1 1] UseAttack
  (if (`self.IsAttacking`)
    (bind (_outhits _returnvalue_2) (`KismetSystemLibrary.SphereTraceMultiForObjects` _returnvalue (+ _returnvalue (* (`self.GetActorUpVector`) (`self.HitboxLength`))) (`self.HitboxRadius`) (`|MakeArray` "ObjectTypeQuery3" :!type "EObjectTypeQuery Enum") false ActorsToIgnore "ForOneFrame"))
    (if _returnvalue_2
      (for _array_element _outhits
        (bind (_bblockinghit _binitialoverlap _time _distance _location _impactpoint _normal _impactnormal _physmat _hitactor) (`GameplayStatics.BreakHitResult` _array_element))
        (if (`Actor.bCanBeDamaged` _hitactor)
          (bind _asbp_player_v3 (cast `/Game/Blueprints/Player/BP_PlayerV3` _hitactor)
            (:`then`
              (if (`/Game/Blueprints/Player/BP_PlayerV3.isUsingSpecialHitbox` _asbp_player_v3)
                (if (`PrimitiveComponent.IsOverlappingComponent` (`self.WeaponMesh`) (`/Game/Blueprints/Player/BP_PlayerV3.SpecialHitbox` _asbp_player_v3))
                  (`KismetSystemLibrary.PrintString` "special overlap")
                  (`self.Deal Damage And Update List` _hitactor))
                (elif (`PrimitiveComponent.IsOverlappingComponent` (`self.WeaponMesh`) (`Character.CapsuleComponent` _asbp_player_v3))
                  (`KismetSystemLibrary.PrintString` "normal overlap")
                  (`self.Deal Damage And Update List` _hitactor))))
            (:`CastFailed`
              (`self.Deal Damage And Update List` _hitactor))))))))

(event `Configure Ignore Classes`
  (params (`Added Classes` :type "Array of Actor Class Reference"))
  ;[1 1 1] Configure Ignore Classes
  (for _array_element `Added Classes`
    (`KismetArrayLibrary.Array_Add` (`self.ActorClassesToIgnore`) _array_element)))

(event `Deal Damage And Update List`
  (params (ActorToDamage :type "Actor Object Reference"))
  ;[1 1 1] Damage
  (`GameplayStatics.ApplyDamage` ActorToDamage (`self.currentDamage`) null self)
  (`KismetArrayLibrary.Array_Add` (`self.ActorsToIgnore`) ActorToDamage))

(event `self.WeaponHitbox.OnComponentBeginOverlap`
  (params (OverlappedComponent :type "PrimitiveComponent Object Reference") (OtherActor :type "Actor Object Reference") (OtherComp :type "PrimitiveComponent Object Reference") (OtherBodyIndex :type Integer) (bFromSweep :type Boolean) (SweepResult :type "HitResult Structure (by ref)"))
  (`self.ProcessNewOverlap` OtherActor OtherComp))

(event `self.ClearActorClassIgnore`
  (`KismetArrayLibrary.Array_Clear` (`self.ActorClassesToIgnore`))
  (`KismetArrayLibrary.Array_Clear` (`self.ActorsToIgnore`)))

(fn `AddActorClassIgnore`
  (params (classToAdd :type "Actor Class Reference"))
  (returns (ReturnValue :type "Array of Actor Class Reference"))
  (bind _actorclassestoignore (`self.ActorClassesToIgnore`))
  (`KismetArrayLibrary.Array_Add` (`self.ActorClassesToIgnore`) classToAdd)
  (`self.Set Ignore Actors` _actorclassestoignore)
  (return _actorclassestoignore))

(fn `CheckExistingOverlaps`
  (for _array_element (`PrimitiveComponent.GetOverlappingActors` (`self.WeaponHitbox`) "/Script/Engine.Pawn")
    (if (and (not (`KismetArrayLibrary.Array_Contains` (`self.ActorsToIgnore`) _array_element)) (not (`KismetArrayLibrary.Array_Contains` (`self.OverlappedActors`) _array_element)))
      (if (`Actor.bCanBeDamaged` _array_element)
        (`KismetArrayLibrary.Array_Add` (`self.OverlappedActors`) _array_element)))))

(fn `GetBaseDamageToUse`
  (params (animClassToUse :type "AnimMontage Object Reference"))
  (returns (damage :type "Float (double-precision)"))
  (bind _animclasstouse (`local.animClassToUse`))
  (if (or (or (`KismetArrayLibrary.Array_Contains` (`self.rightSwingSequence`) _animclasstouse) (== _animclasstouse (`self.rightHeavySwingAnim`))) (== _animclasstouse (`self.rightDodgeSwingAnim`)))
    (return (`self.weaponSlashRawDamage`))
    (else
      (return (`self.weaponStabRawDamage`)))))

(fn `ProcessNewOverlap`
  (params (InOtherActor :type "Actor Object Reference") (InOtherComp :type "PrimitiveComponent Object Reference"))
  (if (`self.IsAttacking`)
    (bind _asbp_player_v3 (cast `/Game/Blueprints/Player/BP_PlayerV3` (`local.InOtherActor`))
      (:`then`
        (if (== (`/Game/Blueprints/Player/BP_PlayerV3.currentDamageHitbox` _asbp_player_v3) (`local.InOtherComp`))
          (if (and (not (`KismetArrayLibrary.Array_Contains` (`self.ActorsToIgnore`) (`local.InOtherActor`))) (not (`KismetArrayLibrary.Array_Contains` (`self.OverlappedActors`) (`local.InOtherActor`)))) :!label _label
            (if (`Actor.bCanBeDamaged` (`local.InOtherActor`))
              (`KismetArrayLibrary.Array_Add` (`self.OverlappedActors`) (`local.InOtherActor`))))))
      (:`CastFailed`
        (goto _label)))))

(fn `RemoveActorClassIgnore`
  (params (classToRemove :type "Actor Class Reference"))
  (returns (ReturnValue :type "Array of Actor Class Reference"))
  (bind _actorclassestoignore (`self.ActorClassesToIgnore`))
  (`KismetArrayLibrary.Array_RemoveItem` (`self.ActorClassesToIgnore`) classToRemove)
  (`self.Set Ignore Actors` _actorclassestoignore)
  (return _actorclassestoignore))

(fn `SetCurrentDamage`
  (params (isHeavyAttack :type Boolean) (isJumpAttack :type Boolean) (isDodgeAttack :type Boolean) (isOffhandAttack :type Boolean) (animToCheck :type "AnimMontage Object Reference"))
  (locals (selectedBaseDamage :type "Float (double-precision)"))
  (bind _damage (`self.GetBaseDamageToUse` animToCheck))
  (set `local.selectedBaseDamage` _damage)
  (if (`local.isHeavyAttack`)
    (set `self.currentDamage` (* (+ (`local.selectedBaseDamage`) (* (`self.weaponLevel`) (`self.weaponDamageUpPerLevel`))) (`self.weaponHeavyAttackMultiplier`)))
    (elif (`local.isJumpAttack`)
      (set `self.currentDamage` (* (+ (`local.selectedBaseDamage`) (* (`self.weaponLevel`) (`self.weaponDamageUpPerLevel`))) (`self.weaponJumpAttackMultiplier`)))
      (elif (`local.isDodgeAttack`)
        (set `self.currentDamage` (* (+ (`local.selectedBaseDamage`) (* (`self.weaponLevel`) (`self.weaponDamageUpPerLevel`))) (`self.weaponDodgeAttackMultiplier`)))
        (elif (`local.isOffhandAttack`)
          (set `self.currentDamage` (* (+ (`self.weaponOffhandRawDamage`) (* (`self.weaponLevel`) (`self.weaponDamageUpPerLevel`))) (`self.weaponOffhandAttackMultiplier`)))
          (else
            (set `self.currentDamage` (* (+ (`local.selectedBaseDamage`) (* (`self.weaponLevel`) (`self.weaponDamageUpPerLevel`))) 1.0))))))))

(fn `TickProcessHitActors`
  (for _array_element (`self.OverlappedActors`)
    (`self.Deal Damage And Update List` _array_element))
  (`KismetArrayLibrary.Array_Clear` (`self.OverlappedActors`)))

(fn `UserConstructionScript`)