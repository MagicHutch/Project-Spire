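; BP_ItemPickupV2 is a world pickup that gives the player the items and quantities in its ItemToGive map.
; Overlap registers it as the player's InteractItem and toggles the HUD interact prompt.
; Interact sorts each valid item into the inventory, shows it on the HUD and destroys the actor.
; It records collection by LevelObjectID in GlobalTempData on the GameInstance, so BeginPlay deletes pickups already taken.
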(event `self.ReceiveBeginPlay`
  (bind _asglobal_temp_data (cast `GlobalTempData` (`GameplayStatics.GetGameInstance`)))
  (bind _output_get (set `self.GlobalTempData` _asglobal_temp_data))
  (if (== (`BlueprintMapLibrary.Map_Find` (`GlobalTempData.levelObjectStateData` _output_get) (`self.levelObjectID`)) 1)
    (`self.DeletePickup`)))

(event `self.ReceiveTick`
  (params (DeltaSeconds :type "Float (single-precision)"))
  (if (not (`KismetSystemLibrary.IsValid` (`self.Player`)))
    (bind _asbp_player_v3 (cast `/Game/Blueprints/Player/BP_PlayerV3` (`GameplayStatics.GetPlayerPawn` 0)))
    (set `self.Player` _asbp_player_v3)))

(event `self.ReceiveActorBeginOverlap`
  (params (OtherActor :type "Actor Object Reference"))
  (bind _asbp_player_v3 (cast `/Game/Blueprints/Player/BP_PlayerV3` OtherActor))
  (set `/Game/Blueprints/Player/BP_PlayerV3.InteractItem` self _asbp_player_v3)
  (bind _asui_hud (cast `/Game/UI/NewUI/Screens/UI_HUD` (`BlueprintMapLibrary.Map_Find` (`/Game/UI/NewUI/WB_MasterUI.ScreensMap` (`/Game/Blueprints/Player/BP_PlayerV3.UI` _asbp_player_v3)) "NewEnumerator0")))
  (`/Game/UI/NewUI/Screens/UI_HUD.Show Interact Prompt` _asui_hud (`self.interactPrompt`) "/Game/ThirdPerson/Input/Actions/IA_Interact.IA_Interact" true))

(event `self.ReceiveActorEndOverlap`
  (params (OtherActor :type "Actor Object Reference"))
  (bind _asbp_player_v3 (cast `/Game/Blueprints/Player/BP_PlayerV3` OtherActor))
  (if (== (`/Game/Blueprints/Player/BP_PlayerV3.InteractItem` _asbp_player_v3) self)
    (set `/Game/Blueprints/Player/BP_PlayerV3.InteractItem` null _asbp_player_v3)
    (bind _asui_hud (cast `/Game/UI/NewUI/Screens/UI_HUD` (`BlueprintMapLibrary.Map_Find` (`/Game/UI/NewUI/WB_MasterUI.ScreensMap` (`/Game/Blueprints/Player/BP_PlayerV3.UI` _asbp_player_v3)) "NewEnumerator0")))
    (`/Game/UI/NewUI/Screens/UI_HUD.Hide Interact Prompt` _asui_hud)))

(event `self.Interact`
  (bind _itemtogive (`self.ItemToGive`))
  (bind _itemtogive_2 (`self.ItemToGive`))
  (bind _keys (`BlueprintMapLibrary.Map_Keys` _itemtogive_2))
  (for (_array_element _array_index) _keys
    (if (`KismetSystemLibrary.IsValidClass` _array_element)
      (`PlayerInventory.SortIncomingObject` (`/Game/Blueprints/Player/BP_PlayerV3.PlayerInventory` (`self.Player`)) _array_element (`BlueprintMapLibrary.Map_Find` _itemtogive_2 _array_element) null)
      (`BlueprintMapLibrary.Map_Add` (`GlobalTempData.levelObjectStateData` (`self.GlobalTempData`)) (`self.levelObjectID`) 1)
      (bind _asui_hud (cast `/Game/UI/NewUI/Screens/UI_HUD` (`BlueprintMapLibrary.Map_Find` (`/Game/UI/NewUI/WB_MasterUI.ScreensMap` (`/Game/Blueprints/Player/BP_PlayerV3.UI` (`self.Player`))) "NewEnumerator0")))
      (bind _keys_2 (`BlueprintMapLibrary.Map_Keys` _itemtogive))
      (bind _output (`|GetArrayItem` _keys_2 _array_index))
      (`/Game/UI/NewUI/Screens/UI_HUD.AddRecentDisplayItem` _asui_hud _output (`BlueprintMapLibrary.Map_Find` _itemtogive _output))
      (`self.K2_DestroyActor`))))

(event `DeletePickup`
  (`self.K2_DestroyActor`))

(fn `UserConstructionScript`)