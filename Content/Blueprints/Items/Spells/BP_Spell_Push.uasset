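; Push spell that launches the player's targeted physics object away from them with a slight upward lift.
; While active, Tick resets the object's velocity and reapplies a steadily decaying impulse until release or depletion.
; On release, a camera trace for an enemy redirects the object at it with double initial impulse, then the player returns to default state.
; An early release is latched, and debug prints and lines remain active.
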(event `self.ReceiveBeginPlay`
  (bind _asbp_player_v3 (cast `/Game/Blueprints/Player/BP_PlayerV3` (`GameplayStatics.GetPlayerPawn` 0)))
  (set `self.playerReference` _asbp_player_v3))

(event `self.ReceiveTick`
  (params (DeltaSeconds :type "Float (single-precision)"))
  (`KismetSystemLibrary.PrintString` (`KismetTextLibrary.Conv_TextToString` (`|FormatText` "Player has released spell button: {0}" (`self.hasBeenReleased`))) true true (struct :`G` 0.66 :`B` 1.0 :`A` 1.0) 2.0 "releaase")
  (if (`self.isCurrentlyInUse`)
    (`self.useSpellTick` DeltaSeconds)))

(event `self.useSpell`
  (if (`KismetSystemLibrary.IsValid` (`self.objectToManip`))
    (bind _outimpulsevector (`self.CalculateLaunchImpulse_0` (`self.K2_GetActorLocation` (`self.playerReference`)) (`SceneComponent.K2_GetComponentLocation` (`/Game/Blueprints/IntersectionObjects/BP_TestIntersectionObject.Cube` (`self.objectToManip`))) 0.5))
    (set `self.directionToLaunch` _outimpulsevector)
    (bind _output_get (set `self.currentImpulse` (`self.initialImpulse`)))
    (`self.SetObjectImpulse` _output_get)
    (set `self.isCurrentlyInUse` true)
    (if (`self.hasBeenReleased`)
      (`self.useSpellReleased`))
    (else
      (`self.useSpellAbort`))))

(event `self.useSpellTick`
  (params (tickLength :type "Float (single-precision)"))
  (if (and (>= (`self.currentImpulse`) 0.0) (`KismetSystemLibrary.IsValid` (`self.objectToManip`)))
    (`self.SetObjectImpulse` (`self.currentImpulse`))
    (set `self.currentImpulse` (- (`self.currentImpulse`) (* (`self.impulseReducePerSecond`) tickLength)))
    (else
      (`self.useSpellReleased`))))

(event `self.useSpellReleased`
  (if (`self.isCurrentlyInUse`)
    (set `self.hasBeenReleased` false)
    (`self.CheckEnemyInSight` 3000.0)
    (`self.SetObjectImpulse` (`self.currentImpulse`))
    (set `self.isCurrentlyInUse` false)
    (`self.ReturnToBase`)
    (else
      (set `self.hasBeenReleased` true))))

(event `self.useSpellAbort`
  (`self.SetObjectImpulse` 0.0)
  (set `self.hasBeenReleased` false)
  (set `self.isCurrentlyInUse` false))

(event `self.useSpellImmediate`
  (bind _currentintersectionobject (`/Game/Blueprints/Player/BP_PlayerV3.currentIntersectionObject` (`self.playerReference`)))
  (if (`KismetSystemLibrary.IsValid` _currentintersectionobject)
    (set `self.objectToManip` _currentintersectionobject)
    (else
      (`self.useSpellAbort`))))

(fn `CalculateLaunchImpulse`
  (params (sourceActor :type "Actor Object Reference") (targetActor :type "Actor Object Reference") (verticalImpulse :type "Float (double-precision)"))
  (returns (outImpulseVector :type "Vector Structure"))
  (locals (positionOne :type "Vector Structure") (positionTwo :type "Vector Structure") (horizontalVector :type "Vector Structure"))
  (bind (_positionone_x _positionone_y) (`KismetMathLibrary.BreakVector` (`local.positionOne`)))
  (bind (_positiontwo_x _positiontwo_y) (`KismetMathLibrary.BreakVector` (`local.positionTwo`)))
  (bind (_returnvalue_x _returnvalue_y) (`KismetMathLibrary.BreakVector` (`KismetMathLibrary.Normal` (`KismetMathLibrary.MakeVector` (- _positiontwo_x _positionone_x) (- _positiontwo_y _positionone_y)))))
  (set `local.positionOne` (`self.K2_GetActorLocation` sourceActor))
  (set `local.positionTwo` (`self.K2_GetActorLocation` targetActor))
  (bind _output_get (set `local.horizontalVector` (`KismetMathLibrary.MakeVector` _returnvalue_x _returnvalue_y (`local.verticalImpulse`))))
  (`KismetSystemLibrary.DrawDebugLine` (`local.positionOne`) (`local.positionTwo`) (struct :`R` 1.0 :`B` 0.085073 :`A` 1.0) 2.0 5.0)
  (return _output_get))

(fn `CalculateLaunchImpulse_0`
  (params (sourceActorPosition :type "Vector Structure") (targetActorPosition :type "Vector Structure") (verticalImpulse :type "Float (double-precision)"))
  (returns (outImpulseVector :type "Vector Structure"))
  (locals (positionOne :type "Vector Structure") (positionTwo :type "Vector Structure") (horizontalVector :type "Vector Structure"))
  (bind (_positionone_x _positionone_y) (`KismetMathLibrary.BreakVector` (`local.positionOne`)))
  (bind (_positiontwo_x _positiontwo_y) (`KismetMathLibrary.BreakVector` (`local.positionTwo`)))
  (bind (_returnvalue_x _returnvalue_y) (`KismetMathLibrary.BreakVector` (`KismetMathLibrary.Normal` (`KismetMathLibrary.MakeVector` (- _positiontwo_x _positionone_x) (- _positiontwo_y _positionone_y)))))
  (set `local.positionOne` sourceActorPosition)
  (set `local.positionTwo` targetActorPosition)
  (bind _output_get (set `local.horizontalVector` (`KismetMathLibrary.MakeVector` _returnvalue_x _returnvalue_y (`local.verticalImpulse`))))
  (`KismetSystemLibrary.DrawDebugLine` (`local.positionOne`) (`local.positionTwo`) (struct :`R` 1.0 :`B` 0.085073 :`A` 1.0) 2.0 5.0)
  (return _output_get))

(fn `CheckEnemyInSight`
  (params (lengthToCheck :type "Float (double-precision)"))
  (bind _camera (`/Game/Blueprints/Player/BP_PlayerV3.Camera` (`self.playerReference`)))
  (bind _returnvalue (`SceneComponent.K2_GetComponentLocation` _camera))
  (bind (_outhit _returnvalue_2) (`KismetSystemLibrary.LineTraceSingleForObjects` _returnvalue (+ _returnvalue (* (`SceneComponent.GetForwardVector` _camera) lengthToCheck)) (`|MakeArray` "ObjectTypeQuery3" :!type "EObjectTypeQuery Enum") false (`|MakeArray` (`self.playerReference`) :!type "Actor Object Reference") "ForDuration"))
  (if _returnvalue_2
    (bind _asenemy_character (cast `EnemyCharacter` (`.HitActor` (`GameplayStatics.BreakHitResult` _outhit))))
    (bind _outimpulsevector (`self.CalculateLaunchImpulse_0` (`SceneComponent.K2_GetComponentLocation` (`/Game/Blueprints/IntersectionObjects/BP_TestIntersectionObject.Cube` (`self.objectToManip`))) (`self.K2_GetActorLocation` _asenemy_character)))
    (set `self.directionToLaunch` _outimpulsevector)
    (`KismetSystemLibrary.PrintString` "enemy detected")
    (set `self.currentImpulse` (* (`self.initialImpulse`) 2.0))))

(fn `ReturnToBase`
  (bind _playerreference (`self.playerReference`))
  (`/Game/Blueprints/Player/BP_PlayerV3.SwitchState` _playerreference (`/Game/Blueprints/Player/BP_PlayerV3.PA_Default` _playerreference)))

(fn `SetObjectImpulse`
  (params (impulseMagnitude :type "Float (double-precision)"))
  (bind _cube (`/Game/Blueprints/IntersectionObjects/BP_TestIntersectionObject.Cube` (`self.objectToManip`)))
  (`PrimitiveComponent.SetPhysicsLinearVelocity` _cube (0.0 0.0 0.0) false "None")
  (`PrimitiveComponent.AddImpulse` _cube (* (`self.directionToLaunch`) (`local.impulseMagnitude`)) "None" false))

(fn `UseMana`
  (bind _asbp_player_v3 (cast `/Game/Blueprints/Player/BP_PlayerV3` (`GameplayStatics.GetPlayerPawn` 0)))
  (bind _stats (`PlayerControllerV2.stats` _asbp_player_v3))
  (set `CharacterStats.currentMana` (- (`CharacterStats.currentMana` _stats) (`self.spellCost`)) _stats))

(fn `UserConstructionScript`)