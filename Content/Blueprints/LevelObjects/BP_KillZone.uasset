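; BP_KillZone is a level object that deals lethal-scale damage to the player on contact.
; On BeginPlay it caches player pawn 0 as a BP_PlayerV3 reference.
; When that player begins overlapping the Cube component, it applies damage equal to the player's maximum health from Stats, ignoring all other actors.
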(event `self.ReceiveBeginPlay`
  (bind _asbp_player_v3 (cast `/Game/Blueprints/Player/BP_PlayerV3` (`GameplayStatics.GetPlayerPawn` 0)))
  (set `self.player` _asbp_player_v3))

(event `self.Cube.OnComponentBeginOverlap`
  (params (OverlappedComponent :type "PrimitiveComponent Object Reference") (OtherActor :type "Actor Object Reference") (OtherComp :type "PrimitiveComponent Object Reference") (OtherBodyIndex :type Integer) (bFromSweep :type Boolean) (SweepResult :type "HitResult Structure (by ref)"))
  (bind _player (`self.player`))
  (if (== OtherActor _player)
    (`GameplayStatics.ApplyDamage` _player (`CharacterStats.maximumHealth` (`PlayerControllerV2.stats` _player)) null self)))

(fn `UserConstructionScript`)