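; Boss fog gate that the player walks through to start a boss encounter.
; Its trigger registers it as the player's interact item and shows a HUD prompt while its saved state is 0.
; Interacting turns the player to a set yaw, starts the fog-gate walk state and aggros the linked boss.
; Once GlobalTempData marks its ID as 1, checked at BeginPlay and on Tick, it hides the gate and removes its collision.
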(event `self.ReceiveBeginPlay`
  (bind _asglobal_temp_data (cast `GlobalTempData` (`GameplayStatics.GetGameInstance`)))
  (bind _output_get (set `self.globalTempData` _asglobal_temp_data))
  (bind _value (`BlueprintMapLibrary.Map_Find` (`GlobalTempData.levelObjectStateData` _output_get) (`self.levelObjectID`)))
  (`KismetSystemLibrary.PrintString` (`KismetStringLibrary.Conv_IntToString` _value))
  (if (== _value 1)
    (`self.DisableGate`))
  (bind _asbp_player_v3 (cast `/Game/Blueprints/Player/BP_PlayerV3` (`GameplayStatics.GetPlayerPawn` 0)))
  (set `self.Player` _asbp_player_v3))

(event `self.ReceiveTick`
  (params (DeltaSeconds :type "Float (single-precision)"))
  (if (and (`SceneComponent.bVisible` (`self.Gate`)) (== (`BlueprintMapLibrary.Map_Find` (`GlobalTempData.levelObjectStateData` (`self.globalTempData`)) (`self.levelObjectID`)) 1))
    (`self.DisableGate`)))

(event `self.Interact`
  (bind _player (`self.Player`))
  (bind (_returnvalue_roll _returnvalue_pitch) (`KismetMathLibrary.BreakRotator` (`self.K2_GetActorRotation` _player)))
  (`self.K2_SetActorRotation` _player (`KismetMathLibrary.MakeRotator` _returnvalue_roll _returnvalue_pitch (`self.playerOrientation`)) false)
  (`/Game/Blueprints/Player/BP_PlayerV3.SwitchState` _player (`/Game/Blueprints/Player/BP_PlayerV3.PA_FogGateWalk` _player))
  (`/Game/Blueprints/Enemies/BP_EnemyCharacter.BossAggroTrigger` (`self.bossToToggleAggro`)))

(event `self.Trigger.OnComponentBeginOverlap`
  (params (OverlappedComponent :type "PrimitiveComponent Object Reference") (OtherActor :type "Actor Object Reference") (OtherComp :type "PrimitiveComponent Object Reference") (OtherBodyIndex :type Integer) (bFromSweep :type Boolean) (SweepResult :type "HitResult Structure (by ref)"))
  (bind _player (`self.Player`))
  (if (and (== OtherActor _player) (== (`BlueprintMapLibrary.Map_Find` (`GlobalTempData.levelObjectStateData` (`self.globalTempData`)) (`self.levelObjectID`)) 0))
    (set `/Game/Blueprints/Player/BP_PlayerV3.InteractItem` self _player)
    (`self.Show Prompt`)))

(event `self.Trigger.OnComponentEndOverlap`
  (params (OverlappedComponent :type "PrimitiveComponent Object Reference") (OtherActor :type "Actor Object Reference") (OtherComp :type "PrimitiveComponent Object Reference") (OtherBodyIndex :type Integer))
  (bind _player (`self.Player`))
  (if (and (== OtherActor _player) (== (`BlueprintMapLibrary.Map_Find` (`GlobalTempData.levelObjectStateData` (`self.globalTempData`)) (`self.levelObjectID`)) 0))
    (set `/Game/Blueprints/Player/BP_PlayerV3.InteractItem` null _player)
    (`self.Hide Prompt`)))

(event `DisableGate`
  (bind _gate (`self.Gate`))
  (`KismetSystemLibrary.PrintString` "gate done")
  (`PrimitiveComponent.SetCollisionEnabled` _gate "NoCollision")
  (`SceneComponent.SetVisibility` _gate false false))

(event `Show Prompt`
  ;[1 1 1] Prompt Logic
  (bind _newparam (`/Game/UI/NewUI/WB_MasterUI.GetScreenByType` (`/Game/Blueprints/Player/BP_PlayerV3.UI` (`self.Player`)) "NewEnumerator0"))
  (bind _asui_hud (cast `/Game/UI/NewUI/Screens/UI_HUD` _newparam))
  (`/Game/UI/NewUI/Screens/UI_HUD.Show Interact Prompt` _asui_hud (`self.interactPrompt`) null true))

(event `Hide Prompt`
  ;[1 1 1] Prompt Logic
  (bind _newparam (`/Game/UI/NewUI/WB_MasterUI.GetScreenByType` (`/Game/Blueprints/Player/BP_PlayerV3.UI` (`self.Player`)) "NewEnumerator0"))
  (bind _asui_hud (cast `/Game/UI/NewUI/Screens/UI_HUD` _newparam))
  (`/Game/UI/NewUI/Screens/UI_HUD.Hide Interact Prompt` _asui_hud))

(fn `UserConstructionScript`)