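; Lever-and-gate level object: interacting with it once permanently opens the gate by hiding it and disabling its collision.
; The switch volume registers the actor as the player's InteractItem and shows a HUD prompt.
; The message volume also registers it, but shows a "locked by a contraption" notice.
; Flipped state is saved by LevelObjectID in the GlobalTempData game instance and reapplied on BeginPlay.
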(event `self.ReceiveBeginPlay`
  (bind _asglobal_temp_data (cast `GlobalTempData` (`GameplayStatics.GetGameInstance`)))
  (bind _output_get (set `self.GlobalTempData` _asglobal_temp_data))
  (if (== (`BlueprintMapLibrary.Map_Find` (`GlobalTempData.levelObjectStateData` _output_get) (`self.levelObjectID`)) 1)
    (`self.DisableGate`))
  (bind _asbp_player_v3 (cast `/Game/Blueprints/Player/BP_PlayerV3` (`GameplayStatics.GetPlayerPawn` 0)))
  (set `self.PlayerReference` _asbp_player_v3))

(event `self.SwitchObject.OnComponentBeginOverlap`
  (params (OverlappedComponent :type "PrimitiveComponent Object Reference") (OtherActor :type "Actor Object Reference") (OtherComp :type "PrimitiveComponent Object Reference") (OtherBodyIndex :type Integer) (bFromSweep :type Boolean) (SweepResult :type "HitResult Structure (by ref)"))
  (if (and (== OtherActor (`self.PlayerReference`)) (not (`self.isFlipped`)))
    (set `/Game/Blueprints/Player/BP_PlayerV3.InteractItem` self (`self.PlayerReference`))
    (`self.Show Prompt`)))

(event `self.SwitchObject.OnComponentEndOverlap`
  (params (OverlappedComponent :type "PrimitiveComponent Object Reference") (OtherActor :type "Actor Object Reference") (OtherComp :type "PrimitiveComponent Object Reference") (OtherBodyIndex :type Integer))
  (if (== OtherActor (`self.PlayerReference`))
    (set `/Game/Blueprints/Player/BP_PlayerV3.InteractItem` null (`self.PlayerReference`))
    (`self.Hide Prompt`)))

(event `self.Interact`
  (if (not (`self.isFlipped`))
    (`self.DisableGate`)
    (`BlueprintMapLibrary.Map_Add` (`GlobalTempData.levelObjectStateData` (`self.GlobalTempData`)) (`self.levelObjectID`) 1)))

(event `DisableGate`
  (bind _gateobject (`self.GateObject`))
  (`PrimitiveComponent.SetCollisionEnabled` _gateobject "NoCollision")
  (`SceneComponent.SetVisibility` _gateobject false false)
  (set `self.isFlipped` true))

(event `Show Prompt`
  ;[1 1 1] Prompt Logic
  (bind _newparam (`/Game/UI/NewUI/WB_MasterUI.GetScreenByType` (`/Game/Blueprints/Player/BP_PlayerV3.UI` (`self.PlayerReference`)) "NewEnumerator0"))
  (bind _asui_hud (cast `/Game/UI/NewUI/Screens/UI_HUD` _newparam))
  (`/Game/UI/NewUI/Screens/UI_HUD.Show Interact Prompt` _asui_hud (`self.interactPrompt`) null true))

(event `Hide Prompt`
  ;[1 1 1] Prompt Logic
  (bind _newparam (`/Game/UI/NewUI/WB_MasterUI.GetScreenByType` (`/Game/Blueprints/Player/BP_PlayerV3.UI` (`self.PlayerReference`)) "NewEnumerator0"))
  (bind _asui_hud (cast `/Game/UI/NewUI/Screens/UI_HUD` _newparam))
  (`/Game/UI/NewUI/Screens/UI_HUD.Hide Interact Prompt` _asui_hud))

(event `self.MessageObject.OnComponentBeginOverlap`
  (params (OverlappedComponent :type "PrimitiveComponent Object Reference") (OtherActor :type "Actor Object Reference") (OtherComp :type "PrimitiveComponent Object Reference") (OtherBodyIndex :type Integer) (bFromSweep :type Boolean) (SweepResult :type "HitResult Structure (by ref)"))
  (if (and (== OtherActor (`self.PlayerReference`)) (not (`self.isFlipped`)))
    (set `/Game/Blueprints/Player/BP_PlayerV3.InteractItem` self (`self.PlayerReference`))
    (bind _newparam (`/Game/UI/NewUI/WB_MasterUI.GetScreenByType` (`/Game/Blueprints/Player/BP_PlayerV3.UI` (`self.PlayerReference`)) "NewEnumerator0"))
    (bind _asui_hud (cast `/Game/UI/NewUI/Screens/UI_HUD` _newparam))
    (`/Game/UI/NewUI/Screens/UI_HUD.Show Interact Prompt` _asui_hud "LOCKED BY A CONTRAPTION" null false)))

(event `self.MessageObject.OnComponentEndOverlap`
  (params (OverlappedComponent :type "PrimitiveComponent Object Reference") (OtherActor :type "Actor Object Reference") (OtherComp :type "PrimitiveComponent Object Reference") (OtherBodyIndex :type Integer))
  (if (== OtherActor (`self.PlayerReference`))
    (`self.Hide Prompt`)))

(fn `UserConstructionScript`)