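; Climbable ladder level object that the player mounts and dismounts by interacting at either end.
; On BeginPlay it places the top trigger above the top anchor and builds instanced mesh segments to fill the height between anchors.
; Trigger overlaps register it as the player's interact item, toggle the HUD prompt and auto-dismount a climbing player.
; Interacting uses the nearer end to snap the player into the climb state, or exits to default if in use.
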(event `self.ReceiveBeginPlay`
  (bind _asbp_player_v3 (cast `/Game/Blueprints/Player/BP_PlayerV3` (`GameplayStatics.GetPlayerPawn` 0)))
  (set `self.PlayerReference` _asbp_player_v3)
  (`self.PositionTopTrigger`)
  (bind _numberofsegments (`self.CalculateNumberOfSegments`))
  (for _index (range (+ _numberofsegments 1))
    (`self.CreateAndPositionSegment` _index)))

(event `self.ReceiveTick`
  (params (DeltaSeconds :type "Float (single-precision)"))
  (bind _playerreference (`self.PlayerReference`))
  (if (`self.inUse`)
    (if (!= (`/Game/Blueprints/Player/BP_PlayerV3.SelfState` _playerreference) (`/Game/Blueprints/Player/BP_PlayerV3.PA_LadderClimb` _playerreference))
      (set `self.inUse` false))))

(event `self.HideTriggersOnStartup`
  (`SceneComponent.SetVisibility` (`self.BottomAnchorAndTrigger`) false false)
  (`SceneComponent.SetVisibility` (`self.TopAnchor`) false false)
  (`SceneComponent.SetVisibility` (`self.TopTrigger`) false false))

(event `self.Interact`
  (`self.InteractProcess`))

(event `self.BottomAnchorAndTrigger.OnComponentBeginOverlap`
  (params (OverlappedComponent :type "PrimitiveComponent Object Reference") (OtherActor :type "Actor Object Reference") (OtherComp :type "PrimitiveComponent Object Reference") (OtherBodyIndex :type Integer) (bFromSweep :type Boolean) (SweepResult :type "HitResult Structure (by ref)"))
  (bind _playerreference (`self.PlayerReference`))
  ;[1 1 1] Bottom Overlap Logic
  (if (== OtherActor _playerreference)
    (set `/Game/Blueprints/Player/BP_PlayerV3.InteractItem` self _playerreference)
    (`self.Show Prompt`)
    (`self.DismountLadder` (`self.BottomAnchorAndTrigger`))))

(event `self.BottomAnchorAndTrigger.OnComponentEndOverlap`
  (params (OverlappedComponent :type "PrimitiveComponent Object Reference") (OtherActor :type "Actor Object Reference") (OtherComp :type "PrimitiveComponent Object Reference") (OtherBodyIndex :type Integer))
  (bind _playerreference (`self.PlayerReference`))
  ;[1 1 1] Bottom Overlap Logic
  (if (== OtherActor _playerreference)
    (set `/Game/Blueprints/Player/BP_PlayerV3.InteractItem` null _playerreference)
    (`self.Hide Prompt`)))

(event `self.TopTrigger.OnComponentBeginOverlap`
  (params (OverlappedComponent :type "PrimitiveComponent Object Reference") (OtherActor :type "Actor Object Reference") (OtherComp :type "PrimitiveComponent Object Reference") (OtherBodyIndex :type Integer) (bFromSweep :type Boolean) (SweepResult :type "HitResult Structure (by ref)"))
  (bind _playerreference (`self.PlayerReference`))
  ;[1 1 1] Top Overlap Logic
  (if (== OtherActor _playerreference)
    (set `/Game/Blueprints/Player/BP_PlayerV3.InteractItem` self _playerreference)
    (`self.Show Prompt`)
    (`self.DismountLadder` (`self.TopTrigger`))))

(event `self.TopTrigger.OnComponentEndOverlap`
  (params (OverlappedComponent :type "PrimitiveComponent Object Reference") (OtherActor :type "Actor Object Reference") (OtherComp :type "PrimitiveComponent Object Reference") (OtherBodyIndex :type Integer))
  (bind _playerreference (`self.PlayerReference`))
  ;[1 1 1] Top Overlap Logic
  (if (== OtherActor _playerreference)
    (set `/Game/Blueprints/Player/BP_PlayerV3.InteractItem` null _playerreference)
    (`self.Hide Prompt`)))

(event `Show Prompt`
  ;[1 1 1] Prompt Logic
  (bind _newparam (`/Game/UI/NewUI/WB_MasterUI.GetScreenByType` (`/Game/Blueprints/Player/BP_PlayerV3.UI` (`self.PlayerReference`)) "NewEnumerator0"))
  (bind _asui_hud (cast `/Game/UI/NewUI/Screens/UI_HUD` _newparam))
  (`/Game/UI/NewUI/Screens/UI_HUD.Show Interact Prompt` _asui_hud (`self.interactPrompt`)))

(event `Hide Prompt`
  ;[1 1 1] Prompt Logic
  (bind _newparam (`/Game/UI/NewUI/WB_MasterUI.GetScreenByType` (`/Game/Blueprints/Player/BP_PlayerV3.UI` (`self.PlayerReference`)) "NewEnumerator0"))
  (bind _asui_hud (cast `/Game/UI/NewUI/Screens/UI_HUD` _newparam))
  (`/Game/UI/NewUI/Screens/UI_HUD.Hide Interact Prompt` _asui_hud))

(fn `AlignPlayerToLadder`
  (params (snapToTopOfLadder :type Boolean))
  (bind (_returnvalue_roll _returnvalue_pitch _returnvalue_yaw) (`KismetMathLibrary.BreakRotator` (`self.K2_GetActorRotation`)))
  (bind (_returnvalue_roll_2 _returnvalue_pitch_2 _returnvalue_yaw_2) (`KismetMathLibrary.BreakRotator` (`self.K2_GetActorRotation`)))
  (bind (_returnvalue_x _returnvalue_y _returnvalue_z) (`KismetMathLibrary.BreakVector` (`SceneComponent.K2_GetComponentLocation` (`self.BottomAnchorAndTrigger`))))
  (bind (_returnvalue_x_2 _returnvalue_y_2 _returnvalue_z_2) (`KismetMathLibrary.BreakVector` (`SceneComponent.K2_GetComponentLocation` (`self.BottomAnchorAndTrigger`))))
  (if snapToTopOfLadder
    ;[1 1 1] Snap To Bottom
    (`self.K2_SetActorLocationAndRotation` (`self.PlayerReference`) (+ (`KismetMathLibrary.MakeVector` _returnvalue_x_2 _returnvalue_y_2 (+ (+ _returnvalue_z_2 (* (`self.verticalSpacingValue`) (`self.numberOfSegments`))) (`self.playerVerticalTopAdjust`))) (* (`self.GetActorForwardVector`) (`self.playerHorizontalSpacing`))) (`KismetMathLibrary.MakeRotator` 0.0 0.0 _returnvalue_yaw_2) false true)
    (else
      ;[1 1 1] Snap To Bottom
      (`self.K2_SetActorLocationAndRotation` (`self.PlayerReference`) (+ (`KismetMathLibrary.MakeVector` _returnvalue_x _returnvalue_y (+ (+ _returnvalue_z (`CapsuleComponent.GetScaledCapsuleHalfHeight` (`Character.CapsuleComponent` (`self.PlayerReference`)))) (`self.playerVerticalBottomAdjust`))) (* (`self.GetActorForwardVector`) (`self.playerHorizontalSpacing`))) (`KismetMathLibrary.MakeRotator` 0.0 0.0 _returnvalue_yaw) false true))))

(fn `CalculateNumberOfSegments`
  (returns (numberOfSegments :type Integer))
  (bind (_returnvalue_x _returnvalue_y _returnvalue_z) (`KismetMathLibrary.BreakVector` (`SceneComponent.K2_GetComponentLocation` (`self.TopAnchor`))))
  (bind (_returnvalue_x_2 _returnvalue_y_2 _returnvalue_z_2) (`KismetMathLibrary.BreakVector` (`SceneComponent.K2_GetComponentLocation` (`self.BottomAnchorAndTrigger`))))
  (bind _output_get (set `self.numberOfSegments` (`KismetMathLibrary.FCeil` (/ (- _returnvalue_z _returnvalue_z_2) (`self.verticalSpacingValue`)))))
  (return _output_get))

(fn `CreateAndPositionSegment`
  (params (segmentNumber :type Integer))
  (bind (_returnvalue_roll _returnvalue_pitch _returnvalue_yaw) (`KismetMathLibrary.BreakRotator` (`self.K2_GetActorRotation`)))
  (bind (_returnvalue_x _returnvalue_y _returnvalue_z) (`KismetMathLibrary.BreakVector` (`SceneComponent.K2_GetComponentLocation` (`self.BottomAnchorAndTrigger`))))
  (`InstancedStaticMeshComponent.AddInstance` (`self.InstancedStaticMesh`) (`KismetMathLibrary.MakeTransform` (+ (`KismetMathLibrary.MakeVector` _returnvalue_x _returnvalue_y (+ _returnvalue_z (* (`self.verticalSpacingValue`) (+ (`local.segmentNumber`) 1)))) (* (`self.GetActorForwardVector`) (`self.horizontalLadderOffset`))) (`KismetMathLibrary.MakeRotator` 0.0 0.0 _returnvalue_yaw)) true))

(fn `DismountLadder`
  (params (AnchorToUse :type "StaticMeshComponent Object Reference"))
  (bind (_returnvalue_x _returnvalue_y) (`KismetMathLibrary.BreakVector` (`SceneComponent.K2_GetComponentLocation` AnchorToUse)))
  (bind _playerreference (`self.PlayerReference`))
  (bind (_returnvalue_x_2 _returnvalue_y_2 _returnvalue_z) (`KismetMathLibrary.BreakVector` (`self.K2_GetActorLocation` _playerreference)))
  (if (`self.inUse`)
    (`self.K2_SetActorLocation` _playerreference (`KismetMathLibrary.MakeVector` _returnvalue_x _returnvalue_y _returnvalue_z) false true)
    (`KismetArrayLibrary.Array_Clear` (`/Game/Blueprints/Player/BP_PlayerV3.ActionQueue` _playerreference))
    (`/Game/Blueprints/Player/BP_PlayerV3.SwitchState` _playerreference (`/Game/Blueprints/Player/BP_PlayerV3.PA_Default` _playerreference))
    (set `self.inUse` false)))

(fn `InteractProcess`
  (bind _playerreference (`self.PlayerReference`))
  (bind _playerreference_2 (`self.PlayerReference`))
  (bind _playerreference_3 (`self.PlayerReference`))
  (bind _playerreference_4 (`self.PlayerReference`))
  (if (< (`KismetMathLibrary.VSize` (- (`self.K2_GetActorLocation` (`self.PlayerReference`)) (`SceneComponent.K2_GetComponentLocation` (`self.BottomAnchorAndTrigger`)))) (`KismetMathLibrary.VSize` (- (`self.K2_GetActorLocation` (`self.PlayerReference`)) (`SceneComponent.K2_GetComponentLocation` (`self.TopTrigger`)))))
    (if (`self.inUse`)
      ;[1 1 1] Climb Off Ladder (Bottom)
      (`/Game/Blueprints/Player/BP_PlayerV3.SwitchState` _playerreference (`/Game/Blueprints/Player/BP_PlayerV3.PA_Default` _playerreference))
      (set `self.inUse` false)
      (else
        ;[1 1 1] Climb On Ladder (Bottom)
        (`self.AlignPlayerToLadder` false)
        (`/Game/Blueprints/Player/BP_PlayerV3.SwitchState` _playerreference_4 (`/Game/Blueprints/Player/BP_PlayerV3.PA_LadderClimb` _playerreference_4))
        (set `self.inUse` true)))
    (elif (`self.inUse`)
      ;[1 1 1] Climb Off Ladder (Top)
      (`/Game/Blueprints/Player/BP_PlayerV3.SwitchState` _playerreference_2 (`/Game/Blueprints/Player/BP_PlayerV3.PA_Default` _playerreference_2))
      (set `self.inUse` false)
      (else
        ;[1 1 1] Climb On Ladder (Top)
        (`self.AlignPlayerToLadder` true)
        (`/Game/Blueprints/Player/BP_PlayerV3.SwitchState` _playerreference_3 (`/Game/Blueprints/Player/BP_PlayerV3.PA_LadderClimb` _playerreference_3))
        (set `self.inUse` true)))))

(fn `PositionTopTrigger`
  (`SceneComponent.K2_SetWorldLocation` (`self.TopTrigger`) (+ (+ (`SceneComponent.K2_GetComponentLocation` (`self.TopAnchor`)) (`KismetMathLibrary.MakeVector` 0.0 0.0 (+ (* (`CapsuleComponent.GetScaledCapsuleHalfHeight` (`Character.CapsuleComponent` (`self.PlayerReference`))) 2.0) 10.0))) (* (`self.GetActorForwardVector`) (`self.horizontalLadderOffset`))) false true))

(fn `UserConstructionScript`)