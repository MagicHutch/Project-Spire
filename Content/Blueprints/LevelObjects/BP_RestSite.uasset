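; BP_RestSite is an interactable rest point that sends the player to another level to rest.
; Its trigger registers it as the player's interact item and shows a HUD prompt while overlapped, clearing both on exit.
; On interact, it saves the site name, inventory, Or count and resting flag to the GlobalTempData game instance, then opens the configured level by name.
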(event `self.ReceiveBeginPlay`
  (bind _asglobal_temp_data (cast `GlobalTempData` (`GameplayStatics.GetGameInstance`)))
  (set `self.globalTempData` _asglobal_temp_data)
  (bind _asbp_player_v3 (cast `/Game/Blueprints/Player/BP_PlayerV3` (`GameplayStatics.GetPlayerPawn` 0)))
  (set `self.player` _asbp_player_v3))

(event `self.Interact`
  (bind _globaltempdata (`self.globalTempData`))
  (bind _player (`self.player`))
  (set `GlobalTempData.currentRestSite` (`self.siteName`) _globaltempdata)
  (`GlobalTempData.WritePlayerStateToTemporaryData` _globaltempdata (`/Game/Blueprints/Player/BP_PlayerV3.PlayerInventory` _player))
  (set `GlobalTempData.playerCurrentOr` (`PlayerControllerV2.orCount` _player) _globaltempdata)
  (set `GlobalTempData.playerIsResting` true (`self.globalTempData`))
  (`GameplayStatics.OpenLevel` (`self.levelNameToLoad`)))

(event `self.Trigger.OnComponentBeginOverlap`
  (params (OverlappedComponent :type "PrimitiveComponent Object Reference") (OtherActor :type "Actor Object Reference") (OtherComp :type "PrimitiveComponent Object Reference") (OtherBodyIndex :type Integer) (bFromSweep :type Boolean) (SweepResult :type "HitResult Structure (by ref)"))
  ;[1 1 1] Overlap Events
  (if (== OtherActor (`self.player`))
    (set `/Game/Blueprints/Player/BP_PlayerV3.InteractItem` self (`self.player`))
    (`self.Show Prompt`)))

(event `self.Trigger.OnComponentEndOverlap`
  (params (OverlappedComponent :type "PrimitiveComponent Object Reference") (OtherActor :type "Actor Object Reference") (OtherComp :type "PrimitiveComponent Object Reference") (OtherBodyIndex :type Integer))
  ;[1 1 1] Overlap Events
  (if (== OtherActor (`self.player`))
    (set `/Game/Blueprints/Player/BP_PlayerV3.InteractItem` null (`self.player`))
    (`self.Hide Prompt`)))

(event `Show Prompt`
  ;[1 1 1] Prompt Logic
  (bind _newparam (`/Game/UI/NewUI/WB_MasterUI.GetScreenByType` (`/Game/Blueprints/Player/BP_PlayerV3.UI` (`self.player`)) "NewEnumerator0"))
  (bind _asui_hud (cast `/Game/UI/NewUI/Screens/UI_HUD` _newparam))
  (`/Game/UI/NewUI/Screens/UI_HUD.Show Interact Prompt` _asui_hud (`self.interactPrompt`) null true))

(event `Hide Prompt`
  ;[1 1 1] Prompt Logic
  (bind _newparam (`/Game/UI/NewUI/WB_MasterUI.GetScreenByType` (`/Game/Blueprints/Player/BP_PlayerV3.UI` (`self.player`)) "NewEnumerator0"))
  (bind _asui_hud (cast `/Game/UI/NewUI/Screens/UI_HUD` _newparam))
  (`/Game/UI/NewUI/Screens/UI_HUD.Hide Interact Prompt` _asui_hud))

(fn `UserConstructionScript`)