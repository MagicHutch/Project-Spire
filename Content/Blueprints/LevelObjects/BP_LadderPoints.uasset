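; BP_LadderPoints is a level object marking a ladder's top and bottom anchors, showing an interact prompt when the player is at either end.
; It caches the BP_PlayerV3 pawn on BeginPlay, then each anchor's begin and end overlaps with that player trigger ShowPrompt or HidePrompt.
; Both events fetch UI_HUD through the player's UI screen lookup to display or hide the prompt; no climbing logic lives here.
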(event `self.ReceiveBeginPlay`
  (bind _asbp_player_v3 (cast `/Game/Blueprints/Player/BP_PlayerV3` (`GameplayStatics.GetPlayerPawn` 0)))
  (set `self.Player` _asbp_player_v3))

(event `self.TopAnchor.OnComponentBeginOverlap`
  (params (OverlappedComponent :type "PrimitiveComponent Object Reference") (OtherActor :type "Actor Object Reference") (OtherComp :type "PrimitiveComponent Object Reference") (OtherBodyIndex :type Integer) (bFromSweep :type Boolean) (SweepResult :type "HitResult Structure (by ref)"))
  (if (== OtherActor (`self.Player`))
    (`self.Show Prompt`)))

(event `self.TopAnchor.OnComponentEndOverlap`
  (params (OverlappedComponent :type "PrimitiveComponent Object Reference") (OtherActor :type "Actor Object Reference") (OtherComp :type "PrimitiveComponent Object Reference") (OtherBodyIndex :type Integer))
  (if (== OtherActor (`self.Player`))
    (`self.Hide Prompt`)))

(event `self.BottomAnchor.OnComponentBeginOverlap`
  (params (OverlappedComponent :type "PrimitiveComponent Object Reference") (OtherActor :type "Actor Object Reference") (OtherComp :type "PrimitiveComponent Object Reference") (OtherBodyIndex :type Integer) (bFromSweep :type Boolean) (SweepResult :type "HitResult Structure (by ref)"))
  (if (== OtherActor (`self.Player`))
    (`self.Show Prompt`)))

(event `self.BottomAnchor.OnComponentEndOverlap`
  (params (OverlappedComponent :type "PrimitiveComponent Object Reference") (OtherActor :type "Actor Object Reference") (OtherComp :type "PrimitiveComponent Object Reference") (OtherBodyIndex :type Integer))
  (if (== OtherActor (`self.Player`))
    (`self.Hide Prompt`)))

(event `Show Prompt`
  (bind _newparam (`/Game/UI/NewUI/WB_MasterUI.GetScreenByType` (`/Game/Blueprints/Player/BP_PlayerV3.UI` (`self.Player`)) "NewEnumerator0"))
  (bind _asui_hud (cast `/Game/UI/NewUI/Screens/UI_HUD` _newparam))
  (`/Game/UI/NewUI/Screens/UI_HUD.Show Interact Prompt` _asui_hud (`self.interactPrompt`)))

(event `Hide Prompt`
  (bind _newparam (`/Game/UI/NewUI/WB_MasterUI.GetScreenByType` (`/Game/Blueprints/Player/BP_PlayerV3.UI` (`self.Player`)) "NewEnumerator0"))
  (bind _asui_hud (cast `/Game/UI/NewUI/Screens/UI_HUD` _newparam))
  (`/Game/UI/NewUI/Screens/UI_HUD.Hide Interact Prompt` _asui_hud))

(fn `UserConstructionScript`)