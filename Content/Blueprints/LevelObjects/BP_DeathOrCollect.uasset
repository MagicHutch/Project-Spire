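; BP_DeathOrCollect is an interactable pickup that returns an amount of "Or" to the player, placed at the death drop location.
; On BeginPlay it teleports to DeathOrSpawnLocation from GlobalTempData in the game instance and caches the player.
; Its trigger overlap registers it as the player's InteractItem and toggles the HUD interact prompt.
; Interact adds AmountToGive to the player's OrCount and destroys the actor.
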(event `self.ReceiveBeginPlay`
  (bind _asglobal_temp_data (cast `GlobalTempData` (`GameplayStatics.GetGameInstance`)))
  (bind _output_get (set `self.globalTempData` _asglobal_temp_data))
  (`self.K2_SetActorLocation` (`GlobalTempData.deathOrSpawnLocation` _output_get) false true)
  (bind _asbp_player_v3 (cast `/Game/Blueprints/Player/BP_PlayerV3` (`GameplayStatics.GetPlayerPawn` 0)))
  (set `self.player` _asbp_player_v3))

(event `self.Interact`
  (bind _player (`self.player`))
  (set `PlayerControllerV2.orCount` (+ (`PlayerControllerV2.orCount` _player) (`self.amountToGive`)) _player)
  (`self.K2_DestroyActor`))

(event `self.Trigger.OnComponentBeginOverlap`
  (params (OverlappedComponent :type "PrimitiveComponent Object Reference") (OtherActor :type "Actor Object Reference") (OtherComp :type "PrimitiveComponent Object Reference") (OtherBodyIndex :type Integer) (bFromSweep :type Boolean) (SweepResult :type "HitResult Structure (by ref)"))
  (bind _player (`self.player`))
  (if (== OtherActor _player)
    (set `/Game/Blueprints/Player/BP_PlayerV3.InteractItem` self _player)
    (`self.Show Prompt`)))

(event `self.Trigger.OnComponentEndOverlap`
  (params (OverlappedComponent :type "PrimitiveComponent Object Reference") (OtherActor :type "Actor Object Reference") (OtherComp :type "PrimitiveComponent Object Reference") (OtherBodyIndex :type Integer))
  (bind _player (`self.player`))
  (if (== OtherActor _player)
    (set `/Game/Blueprints/Player/BP_PlayerV3.InteractItem` null _player)
    (`self.Hide Prompt`)))

(event `Show Prompt`
  ;[1 1 1] Prompt Logic
  (bind _newparam (`/Game/UI/NewUI/WB_MasterUI.GetScreenByType` (`/Game/Blueprints/Player/BP_PlayerV3.UI` (`self.player`)) "NewEnumerator0"))
  (bind _asui_hud (cast `/Game/UI/NewUI/Screens/UI_HUD` _newparam))
  (`/Game/UI/NewUI/Screens/UI_HUD.Show Interact Prompt` _asui_hud (`self.interactPrompt`)))

(event `Hide Prompt`
  ;[1 1 1] Prompt Logic
  (bind _newparam (`/Game/UI/NewUI/WB_MasterUI.GetScreenByType` (`/Game/Blueprints/Player/BP_PlayerV3.UI` (`self.player`)) "NewEnumerator0"))
  (bind _asui_hud (cast `/Game/UI/NewUI/Screens/UI_HUD` _newparam))
  (`/Game/UI/NewUI/Screens/UI_HUD.Hide Interact Prompt` _asui_hud))

(fn `UserConstructionScript`)