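; BP_FirespitterSpark is a homing spark projectile that pursues the player pawn.
; Each Tick it makes a swept move straight toward the player's current location at SpeedPerSecond, then advances a lifespan timer that destroys it at Duration.
; Static world overlaps destroy it; pawn overlaps destroy it only when the damage check succeeds.
; TrackPlayer offers clamped turn-rate steering, but nothing in this Blueprint calls it.
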(event `self.ReceiveBeginPlay`
  (`parent.ReceiveBeginPlay`))

(event `self.ReceiveActorBeginOverlap`
  (params (OtherActor :type "Actor Object Reference"))
  (`parent.ReceiveActorBeginOverlap` OtherActor))

(event `self.ReceiveTick`
  (params (DeltaSeconds :type "Float (single-precision)"))
  (`parent.ReceiveTick` DeltaSeconds)
  (`self.K2_AddActorWorldOffset` (* (* (`KismetMathLibrary.Normal` (- (`self.K2_GetActorLocation` (`GameplayStatics.GetPlayerPawn` 0)) (`self.K2_GetActorLocation`))) (`self.speedPerSecond`)) DeltaSeconds) true)
  (`self.UpdateLifespanTimer` DeltaSeconds))

(fn `OverlapPawn`
  (params (InOtherActor :type "Actor Object Reference") (InOtherComp :type "PrimitiveComponent Object Reference"))
  (`parent.OverlapPawn` InOtherActor InOtherComp)
  (bind _coulddealdamage (`self.CheckDealDamage` (`local.InOtherActor`) (`local.InOtherComp`) 10.0))
  (if _coulddealdamage
    (`self.K2_DestroyActor`)))

(fn `OverlapWorldStatic`
  (`parent.OverlapWorldStatic`)
  (`self.K2_DestroyActor`))

(fn `TrackPlayer`
  (params (inDeltaTime :type "Float (double-precision)") (maxAdjustPerSecond :type "Float (double-precision)"))
  (bind _maxadjustpersecond (`local.maxAdjustPerSecond`))
  (bind _yawpitchreturn (`self.CalculateTrackAdjust` (`self.K2_GetActorLocation`) (`self.K2_GetActorLocation` (`GameplayStatics.GetPlayerPawn` 0)) _maxadjustpersecond _maxadjustpersecond (`local.inDeltaTime`)))
  (`self.K2_AddActorWorldRotation` (`KismetMathLibrary.MakeRotator` 0.0 (`.Y` (`KismetMathLibrary.BreakVector2D` _yawpitchreturn)) (`KismetMathLibrary.BreakVector2D` _yawpitchreturn)))
  (`self.K2_AddActorWorldOffset` (* (`self.GetActorForwardVector`) (* (`self.speedPerSecond`) (`local.inDeltaTime`))) true))

(fn `UpdateLifespanTimer`
  (params (inDeltaTime :type "Float (double-precision)"))
  (bind _output_get (set `self.lifespan` (+ (`self.lifespan`) (`local.inDeltaTime`))))
  (if (>= _output_get (`self.duration`))
    (`self.K2_DestroyActor`)))

(fn `UserConstructionScript`
  (`parent.UserConstructionScript`))