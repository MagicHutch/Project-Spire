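; BP_WeaponProjectile is a weapon projectile Blueprint that acts as a skeleton for reacting to what the projectile hits.
; Its ProjectileHitbox overlap event checks the other component's collision object type, calling OverlapWorldStatic for WorldStatic or OverlapPawn, with the overlapped actor and component, for Pawn.
; Both handler functions are empty here, leaving only the dispatch logic, and other object types are ignored.
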(event `self.ProjectileHitbox.OnComponentBeginOverlap`
  (params (OverlappedComponent :type "PrimitiveComponent Object Reference") (OtherActor :type "Actor Object Reference") (OtherComp :type "PrimitiveComponent Object Reference") (OtherBodyIndex :type Integer) (bFromSweep :type Boolean) (SweepResult :type "HitResult Structure (by ref)"))
  (if (== (`PrimitiveComponent.GetCollisionObjectType` OtherComp) (`KismetSystemLibrary.MakeLiteralByte` (enumliteral `ECollisionChannel` "ECC_WorldStatic")))
    (`self.OverlapWorldStatic`)
    (elif (== (`PrimitiveComponent.GetCollisionObjectType` OtherComp) (`KismetSystemLibrary.MakeLiteralByte` (enumliteral `ECollisionChannel` "ECC_Pawn")))
      (`self.OverlapPawn` OtherActor OtherComp))))

(fn `OverlapPawn`
  (params (InOtherActor :type "Actor Object Reference") (InOtherComp :type "PrimitiveComponent Object Reference")))

(fn `OverlapWorldStatic`)

(fn `UserConstructionScript`)