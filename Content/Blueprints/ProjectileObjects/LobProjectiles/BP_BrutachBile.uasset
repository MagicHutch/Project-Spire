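; BP_BrutachBile is a lobbed bile projectile that damages pawns it hits or leaves a puddle on world geometry.
; On world-static overlap it spawns a BP_BrutachBilePuddle just above the mesh location and destroys itself.
; On pawn overlap it ignores its source and counts player hits only on the current damage hitbox.
; Hits on damageable pawns apply damage, raise the Despair meter through CharacterStats if present, then destroy the projectile.
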(fn `OverlapPawn`
  (params (InOtherActor :type "Actor Object Reference") (InOtherComp :type "PrimitiveComponent Object Reference"))
  (bind _inotheractor (`local.InOtherActor`))
  (bind _returnvalue (`self.GetComponentByClass` _inotheractor "/Script/MyProject.CharacterStats"))
  (if (not (== InOtherActor (`self.sourceActor`)))
    (bind _asbp_player_v3 (cast `/Game/Blueprints/Player/BP_PlayerV3` (`local.InOtherActor`))
      (:`then`
        (if (== (`local.InOtherComp`) (`/Game/Blueprints/Player/BP_PlayerV3.currentDamageHitbox` _asbp_player_v3))
          (if (`Actor.bCanBeDamaged` (`local.InOtherActor`)) :!label _label
            (`GameplayStatics.ApplyDamage` _inotheractor 20.0 null self)
            (if (`KismetSystemLibrary.IsValid` _returnvalue)
              (`CharacterStats.IncreaseDespairMeter` _returnvalue 30.0))
            (`self.K2_DestroyActor`))))
      (:`CastFailed`
        (goto _label)))))

(fn `OverlapWorldStatic`
  (bind (_returnvalue_x _returnvalue_y _returnvalue_z) (`KismetMathLibrary.BreakVector` (`SceneComponent.K2_GetComponentLocation` (`self.ProjectileMesh`))))
  (`|SpawnActorFromClass` "/Game/Blueprints/AreaOfEffectObjects/BP_BrutachBilePuddle.BP_BrutachBilePuddle_C" (`KismetMathLibrary.MakeTransform` (`KismetMathLibrary.MakeVector` _returnvalue_x _returnvalue_y (+ _returnvalue_z 50.0))) "AlwaysSpawn" "MultiplyWithRoot" null (`self.sourceActor`) null)
  (`self.K2_DestroyActor`))

(fn `UserConstructionScript`
  (`parent.UserConstructionScript`))